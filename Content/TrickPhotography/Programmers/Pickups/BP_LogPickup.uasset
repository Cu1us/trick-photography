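; BP_LogPickup is a log pickup that can be placed into a fireplace slot, with a highlight while hovered.
; Activate traces forward from the camera, with debug drawing on; a slot hit detaches the held log, moves it there, notifies the slot and destroys the pickup.
; LogCollidedWithFireplaceSlot also notifies the slot and destroys the log.
; The log's physics setting is applied one tick after BeginPlay.
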(event `self.ReceiveBeginPlay`
  (`parent.ReceiveBeginPlay`)
  (`KismetSystemLibrary.DelayUntilNextTick`)
  (`PrimitiveComponent.SetSimulatePhysics` (`self.Log`) (`self.bPhysicsEnabledAtPlay`)))

(event `PickupableInterface.Activate`
  (params (cameraTransform :type "Transform Structure") (isCammy :type Boolean))
  (bind (_outhits _returnvalue) (`KismetSystemLibrary.LineTraceMultiByProfile` cameraTransform_Location (+ cameraTransform_Location (* (`KismetMathLibrary.GetForwardVector` cameraTransform_Rotation) 750.0)) "BlockAll" true (`|MakeArray` (`GameplayStatics.GetPlayerCharacter` 0) :!type "Actor Object Reference") "ForDuration" true (struct :`R` 1.0 :`A` 1.0) (struct :`G` 1.0 :`A` 1.0) 1.0))
  (if _returnvalue
    (for _array_element _outhits
      (bind _asbp_fire_place_slot (cast `/Game/TrickPhotography/Programmers/Puzzles/BP_FirePlaceSlot` (`.HitActor` (`GameplayStatics.BreakHitResult` _array_element))))
      (bind _asbp_main_character (cast `/Game/TrickPhotography/Programmers/Core/Player/BP_MainCharacter` (`GameplayStatics.GetPlayerCharacter` 0)))
      (`/Game/TrickPhotography/Programmers/Core/Player/BP_MainCharacter.DetachHeldObject` _asbp_main_character)
      (bind (_returnvalue_location _returnvalue_rotation) (`KismetMathLibrary.BreakTransform` (`self.GetTransform` _asbp_fire_place_slot)))
      (`SceneComponent.K2_SetWorldLocationAndRotation` (`self.Log`) _returnvalue_location _returnvalue_rotation false true)
      (`PickupableInterface.OnDrop` false)
      (`self.K2_AttachToActor` _asbp_fire_place_slot "None" "KeepWorld" "KeepWorld" "KeepWorld")
      (`/Game/TrickPhotography/Programmers/Puzzles/BP_FirePlaceSlot.SetLogInFireplace` _asbp_fire_place_slot)
      (`self.K2_DestroyActor`)
      (break))))

(event `PickupableInterface.OnDrop`
  (params (isCammy :type Boolean))
  (`parent.OnDrop` isCammy))

(event `LogCollidedWithFireplaceSlot`
  (params (FireplaceSlot :type "/Game/TrickPhotography/Programmers/Puzzles/BP_FirePlaceSlot Object Reference"))
  (`/Game/TrickPhotography/Programmers/Puzzles/BP_FirePlaceSlot.SetLogInFireplace` FireplaceSlot)
  (`self.K2_DestroyActor`))

(event `/Game/TrickPhotography/Programmers/Core/Interfaces/BPI_Interactable.HoverEnd`
  (params (HeldItem :type "PickupableInterface Interface") (bIsCammy :type Boolean))
  (`self.SetPPMHighlight` "None"))

(fn `HoverOngoing`
  (params (HeldItem :type "PickupableInterface Interface") (HitComponent :type "PrimitiveComponent Object Reference"))
  (returns (bIsInteractable :type Boolean))
  (return false))

(fn `HoverStart`
  (params (HeldItem :type "PickupableInterface Interface") (HitComponent :type "PrimitiveComponent Object Reference") (bIsCammy :type Boolean))
  (returns (bIsInteractable :type Boolean))
  (`self.SetPPMHighlight` "HighlightPickup")
  (return false))

(fn `UserConstructionScript`)