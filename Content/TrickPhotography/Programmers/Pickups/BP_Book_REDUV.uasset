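; BP_Book_REDUV is a pickup book that can be placed into BP_BookSlot actors and switches to a UV material on a thermal photo.
; Activating it line-traces from the camera, detaches it from the player, snaps it onto the hit slot and registers its PickupID there.
; Picking it up again clears that slot's registration.
; It registers with GM_MainGame as a filterable on BeginPlay and shows a highlight on hover.
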(event `PickupableInterface.Activate`
  (params (cameraTransform :type "Transform Structure") (isCammy :type Boolean))
  (bind (_outhits _returnvalue) (`KismetSystemLibrary.LineTraceMultiByProfile` cameraTransform_Location (+ cameraTransform_Location (* (`KismetMathLibrary.GetForwardVector` cameraTransform_Rotation) 750.0)) "BlockAll" false (`|MakeArray` (`GameplayStatics.GetPlayerCharacter` 0) :!type "Actor Object Reference") "ForDuration" true (struct :`R` 1.0 :`A` 1.0) (struct :`G` 1.0 :`A` 1.0) 1.0))
  (if _returnvalue
    (for _array_element _outhits
      (bind _asbp_book_slot (cast `/Game/TrickPhotography/Programmers/Puzzles/BP_BookSlot` (`.HitActor` (`GameplayStatics.BreakHitResult` _array_element))))
      (bind _asbp_main_character (cast `/Game/TrickPhotography/Programmers/Core/Player/BP_MainCharacter` (`GameplayStatics.GetPlayerCharacter` 0)))
      (`/Game/TrickPhotography/Programmers/Core/Player/BP_MainCharacter.DetachHeldObject` _asbp_main_character)
      (bind (_returnvalue_location _returnvalue_rotation) (`KismetMathLibrary.BreakTransform` (`self.GetTransform` _asbp_book_slot)))
      (`SceneComponent.K2_SetWorldLocationAndRotation` (`self.Book`) _returnvalue_location _returnvalue_rotation false true)
      (`KismetSystemLibrary.PrintString` "ya")
      (`PickupableInterface.OnDrop` false)
      (`PrimitiveComponent.SetSimulatePhysics` (`self.Book`) false)
      (`self.K2_AttachToActor` _asbp_book_slot "None" "KeepWorld" "KeepWorld" "KeepWorld")
      (`/Game/TrickPhotography/Programmers/Puzzles/BP_BookSlot.SetRegisteredBook` _asbp_book_slot (`self.PickupID`))
      (set `self.AttachedSlot` _asbp_book_slot)
      (break))))

(event `PickupableInterface.OnPickup`
  (params (isCammy :type Boolean))
  (bind _attachedslot (`self.AttachedSlot`))
  (`parent.OnPickup` isCammy)
  (`/Engine/EditorBlueprintResources/StandardMacros.IsValid` _attachedslot
    (:`Is Valid`
      (`/Game/TrickPhotography/Programmers/Puzzles/BP_BookSlot.SetRegisteredBook` _attachedslot "")
      (set `self.AttachedSlot` null)
      (`KismetSystemLibrary.PrintString` "Hello"))))

(event `FilterableInterface.OnThermalPhoto`
  (`PrimitiveComponent.SetMaterial` (`self.Book`) 0 (`self.UVMaterial`)))

(event `self.HoverEnd`
  (params (HeldItem :type "PickupableInterface Interface") (bIsCammy :type Boolean))
  (`self.SetPPMHighlight` "None"))

(event `self.ReceiveBeginPlay`
  (bind _asgm_main_game (cast `/Game/TrickPhotography/Programmers/Core/GM_MainGame` (`GameplayStatics.GetGameMode`))
    (:`then`
      (`/Game/TrickPhotography/Programmers/Core/GM_MainGame.RegisterNewFilterable` _asgm_main_game self)
      (`KismetSystemLibrary.PrintString` "sdsadsad" true true (struct :`G` 0.66 :`B` 1.0 :`A` 1.0) 10.0))
    (:`CastFailed`
      (`KismetSystemLibrary.PrintString` "fadsfds" true true (struct :`G` 0.66 :`B` 1.0 :`A` 1.0) 10.0))))

(fn `HoverOngoing`
  (params (HeldItem :type "PickupableInterface Interface") (HitComponent :type "PrimitiveComponent Object Reference"))
  (returns (bIsInteractable :type Boolean))
  (return false))

(fn `HoverStart`
  (params (HeldItem :type "PickupableInterface Interface") (HitComponent :type "PrimitiveComponent Object Reference") (bIsCammy :type Boolean))
  (returns (bIsInteractable :type Boolean))
  (`self.SetPPMHighlight` "HighlightPickup")
  (return false))

(fn `UserConstructionScript`)