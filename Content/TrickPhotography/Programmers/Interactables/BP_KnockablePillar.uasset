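; Interactable pillar that the player can knock over, under a "BONK IT!" prompt, to drop a Polaroid pack.
; On BeginPlay it spawns the pack, attaches it to a socket on the pillar's skeletal mesh and turns its physics off.
; Interacting plays the fall animation, then a short fixed delay turns on the pack's physics.
; A montage notify route to the same release exists but is unconnected.
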(event `self.ReceiveBeginPlay`
  (bind _returnvalue (`|SpawnActorFromClass` "/Game/TrickPhotography/Programmers/Pickups/BP_PolaroidPack.BP_PolaroidPack_C" (`SceneComponent.K2_GetComponentToWorld` (`self.PolaroidPos`)) "Undefined" "MultiplyWithRoot" null null))
  (`self.K2_AttachToComponent` _returnvalue (`self.PillarSkeletalMesh`) "PolaroidSocket" "KeepWorld" "KeepWorld" "KeepWorld" true)
  (`PrimitiveComponent.SetSimulatePhysics` (`/Game/TrickPhotography/Programmers/Pickups/BP_PolaroidPack.Pack` _returnvalue) false))

(event `/Game/TrickPhotography/Programmers/Core/Interfaces/BPI_Interactable.InteractStart`
  (params (HeldItem :type "PickupableInterface Interface") (bIsCammy :type Boolean) (HitComponent :type "PrimitiveComponent Object Reference"))
  (`SkeletalMeshComponent.PlayAnimation` (`self.PillarSkeletalMesh`) "/Game/TrickPhotography/Art/Enviroment/Meshes/PillarFallMontage.PillarFallMontage" false)
  (`KismetSystemLibrary.Delay` 0.5)
  (`PrimitiveComponent.SetSimulatePhysics` (`/Game/TrickPhotography/Programmers/Pickups/BP_PolaroidPack.Pack` (stale `self.ReceiveBeginPlay` _returnvalue)) true))

(event `KickMe`)

(event `/Game/TrickPhotography/Programmers/Core/Interfaces/BPI_Interactable.HoverEnd`
  (params (HeldItem :type "PickupableInterface Interface") (bIsCammy :type Boolean)))

(fn `GetInteractionType`
  (params (bIsCammy :type Boolean) (HitComponent :type "PrimitiveComponent Object Reference"))
  (returns (Type :type "/Game/TrickPhotography/Programmers/Enums/EPlayerInteractionState Enum") (CustomInteractTooltip :type Text))
  (return "NewEnumerator2" "BONK IT!"))

(fn `HoverOngoing`
  (params (HeldItem :type "PickupableInterface Interface") (HitComponent :type "PrimitiveComponent Object Reference"))
  (returns (bIsInteractable :type Boolean))
  (return false))

(fn `HoverStart`
  (params (HeldItem :type "PickupableInterface Interface") (HitComponent :type "PrimitiveComponent Object Reference") (bIsCammy :type Boolean))
  (returns (bIsInteractable :type Boolean))
  (return false))

(fn `UserConstructionScript`)