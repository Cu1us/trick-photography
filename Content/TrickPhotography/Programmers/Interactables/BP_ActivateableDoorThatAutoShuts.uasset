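; An activatable door that swings open when activated and shuts itself when the player character leaves an assigned trigger.
; BeginPlay caches the starting yaw and binds the end-overlap of CloseOnExitTrigger, which calls Deactivate for BP_MainCharacter.
; Separate Open and Close timelines drive the actor's yaw as an offset from that cached rotation.
; Debug prints remain on overlap, activation and close, plus an unused leftover node chain.
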(event `self.ReceiveBeginPlay`
  (bind (_returnvalue_roll _returnvalue_pitch _returnvalue_yaw) (`KismetMathLibrary.BreakRotator` (`self.K2_GetActorRotation`)))
  (bind _closeonexittrigger (`self.CloseOnExitTrigger`))
  (`parent.ReceiveBeginPlay`)
  (set `self.InitialRot` _returnvalue_yaw)
  (`/Engine/EditorBlueprintResources/StandardMacros.IsValid` _closeonexittrigger
    (:`Is Valid`
      (add `self.OnActorEndOverlap` _closeonexittrigger (delegate `OnActorEndOverlap_Event`)))))

(event `OnActorEndOverlap_Event` :!signature `self.OnActorEndOverlap`
  (params (OverlappedActor :type "Actor Object Reference") (OtherActor :type "Actor Object Reference"))
  (`KismetSystemLibrary.PrintString` "dadwadesfa")
  (cast `/Game/TrickPhotography/Programmers/Core/Player/BP_MainCharacter` OtherActor)
  (`/Game/TrickPhotography/Programmers/Core/Interfaces/BPI_Activatable.Deactivate`))

(event `self.Activate`
  (bind (_returnvalue_roll _returnvalue_pitch) (`KismetMathLibrary.BreakRotator` (`self.K2_GetActorRotation`)))
  (`KismetSystemLibrary.PrintString` "Activated")
  (bind (_direction _z) (`Timeline|Open`)
    (:`Update`
      (`self.K2_SetActorRotation` (`KismetMathLibrary.MakeRotator` _returnvalue_roll _returnvalue_pitch (+ _z (`self.InitialRot`)))))))

(event `/Game/TrickPhotography/Programmers/Core/Interfaces/BPI_Activatable.Deactivate`
  (bind (_returnvalue_roll _returnvalue_pitch) (`KismetMathLibrary.BreakRotator` (`self.K2_GetActorRotation`)))
  (`parent.Deactivate`)
  (bind (_direction _z) (`Timeline|Close`)
    (:`Update`
      (`self.K2_SetActorRotation` (`KismetMathLibrary.MakeRotator` _returnvalue_roll _returnvalue_pitch (+ _z (`self.InitialRot`)))))
    (:`Finished`
      (`KismetSystemLibrary.PrintString` "closed"))))

(fn `UserConstructionScript`
  (`parent.UserConstructionScript`))