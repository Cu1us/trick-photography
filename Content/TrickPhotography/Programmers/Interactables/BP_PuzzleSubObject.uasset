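; BP_PuzzleSubObject is an interactable piece of a larger puzzle that reports interactions to its PuzzleMainObject.
; InteractStart passes itself to that main object, if valid, through ObjectInteractedWith.
; UpdateActivatedStatus stores whether the piece is properly activated and swaps the FilterStaticMesh material between glowing and plain idol variants.
; Both hover functions simply return false.
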(event `/Game/TrickPhotography/Programmers/Core/Interfaces/BPI_Interactable.InteractStart`
  (params (HeldItem :type "PickupableInterface Interface") (bIsCammy :type Boolean) (HitComponent :type "PrimitiveComponent Object Reference"))
  (bind _puzzlemainobject (`self.PuzzleMainObject`))
  (`/Engine/EditorBlueprintResources/StandardMacros.IsValid` _puzzlemainobject
    (:`Is Valid`
      (`/Game/TrickPhotography/Programmers/Interactables/BP_PuzzleMainObject.ObjectInteractedWith` _puzzlemainobject self))))

(event `UpdateActivatedStatus`
  (params (bSetActivated :type Boolean))
  (bind _output_get (set `self.bObjectActivatedProperly` bSetActivated))
  (if _output_get
    (`PrimitiveComponent.SetMaterial` (`self.FilterStaticMesh`) 0 "/Game/TrickPhotography/Art/Materials/Idols/M_Idol2Glow.M_Idol2Glow")
    (else
      (`PrimitiveComponent.SetMaterial` (`self.FilterStaticMesh`) 0 "/Game/TrickPhotography/Art/Materials/Idols/M_Idol2.M_Idol2"))))

(fn `HoverOngoing`
  (params (HeldItem :type "PickupableInterface Interface") (HitComponent :type "PrimitiveComponent Object Reference"))
  (returns (bIsInteractable :type Boolean))
  (return false))

(fn `HoverStart`
  (params (HeldItem :type "PickupableInterface Interface") (HitComponent :type "PrimitiveComponent Object Reference"))
  (returns (bIsInteractable :type Boolean))
  (return false))

(fn `UserConstructionScript`)