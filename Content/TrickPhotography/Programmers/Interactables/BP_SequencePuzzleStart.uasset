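; Main idol statue of a sequence puzzle that non-Cammy interactors activate, coordinating linked interactables that must be triggered in order.
; Linked pieces report back to it, and it checks order either instantly per step or once all, itself included, are attempted.
; Failure flashes and resets the idols, while success activates the cutscene camera and parent logic.
; Its own activation state swaps glow materials and toggles linked objects via BPI_Activatable or visibility.
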(event `self.ReceiveBeginPlay`
  (bind _sequencedinteractsincludingself (`self.SequencedInteractsIncludingSelf`))
  (`parent.ReceiveBeginPlay`)
  (for _array_element (`self.SequencedInteractables`)
    (set `/Game/TrickPhotography/Programmers/Interactables/BP_SequencePuzzlePieces.PuzzleMainObject` self _array_element))
  (`KismetArrayLibrary.Array_Add` _sequencedinteractsincludingself self)
  (`KismetArrayLibrary.Array_Append` _sequencedinteractsincludingself (`self.SequencedInteractables`))
  (`self.UpdateActivatedStatus` false))

(event `/Game/TrickPhotography/Programmers/Core/Interfaces/BPI_Interactable.InteractStart`
  (params (HeldItem :type "PickupableInterface Interface") (bIsCammy :type Boolean) (HitComponent :type "PrimitiveComponent Object Reference"))
  (if bIsCammy
    _
    (elif (`self.bObjectActivatedProperly`)
      _
      (elif (`self.bPuzzleCompleted`)
        (`KismetSystemLibrary.PrintString` "Already completed")
        (else
          (`self.UpdateActivatedStatus` false true))))))

(event `UpdateActivatedStatus`
  (params (bFailed :type Boolean) (bSetActivated :type Boolean))
  (if bFailed
    (`/Game/TrickPhotography/Programmers/Core/BaseClasses/CustomMacros.DelayableForLoop` 0 5 :!label _label
      (:`LoopBody`
        (`self.SetMaterial` "/Game/TrickPhotography/Art/Materials/Idols/M_Idol1.M_Idol1")
        (`KismetSystemLibrary.Delay` 0.2)
        (`self.SetMaterial` "/Game/TrickPhotography/Art/Materials/Idols/M_Idol1glow.M_Idol1glow")
        (`KismetSystemLibrary.Delay` 0.1)
        (goto _label :!via `CountUp`))
      (:`Completed`
        (`self.SetMaterial` "/Game/TrickPhotography/Art/Materials/Idols/M_Idol1.M_Idol1")
        (set `self.bObjectActivatedProperly` false)
        (`self.UpdateActivatedStatus` false)))
    (else
      (bind _output_get (set `self.bObjectActivatedProperly` bSetActivated))
      (if _output_get
        (`self.SetMaterial` "/Game/TrickPhotography/Art/Materials/Idols/M_Idol1glow.M_Idol1glow")
        (for _array_element (`self.ObjectsToActivateWhenActivated`)
          (bind _asbpi_activatable (cast `/Game/TrickPhotography/Programmers/Core/Interfaces/BPI_Activatable` _array_element)
            (:`then`
              (`/Game/TrickPhotography/Programmers/Core/Interfaces/BPI_Activatable.Activate` _asbpi_activatable))
            (:`CastFailed`
              (`self.SetActorHiddenInGame` _array_element false))))
        (if (not (`self.bResetInstantlyOnFail`))
          (`self.ObjectInteractedWith` null))
        (else
          (`self.SetMaterial` "/Game/TrickPhotography/Art/Materials/Idols/M_Idol1.M_Idol1")
          (for _array_element_2 (`self.ObjectsToActivateWhenActivated`)
            (bind _asbpi_activatable_2 (cast `/Game/TrickPhotography/Programmers/Core/Interfaces/BPI_Activatable` _array_element_2)
              (:`then`
                (`/Game/TrickPhotography/Programmers/Core/Interfaces/BPI_Activatable.Deactivate` _asbpi_activatable_2))
              (:`CastFailed`
                (`self.SetActorHiddenInGame` _array_element_2 true)))))))))

(event `/Game/TrickPhotography/Programmers/Core/Interfaces/BPI_Interactable.HoverEnd`
  (params (HeldItem :type "PickupableInterface Interface") (bIsCammy :type Boolean))
  (`self.SetPPMHighlight` "None"))

(fn `Activate`
  (`/Game/TrickPhotography/Programmers/Core/Interfaces/BPI_Activatable.Activate` (`self.CutSceneCam`))
  (`parent.Activate`))

(fn `GetInteractionType`
  (params (bIsCammy :type Boolean) (HitComponent :type "PrimitiveComponent Object Reference"))
  (returns (Type :type "/Game/TrickPhotography/Programmers/Enums/EPlayerInteractionState Enum") (CustomInteractTooltip :type Text))
  (return "NewEnumerator5" "Activate Statue"))

(fn `HoverOngoing`
  (params (HeldItem :type "PickupableInterface Interface") (HitComponent :type "PrimitiveComponent Object Reference"))
  (returns (bIsInteractable :type Boolean))
  (return false))

(fn `HoverStart`
  (params (HeldItem :type "PickupableInterface Interface") (HitComponent :type "PrimitiveComponent Object Reference") (bIsCammy :type Boolean))
  (returns (bIsInteractable :type Boolean))
  (`self.SetPPMHighlight` "HighlightPickup")
  (return false))

(fn `ObjectInteractedWith`
  (params (SubObjectedInteracted :type "/Game/TrickPhotography/Programmers/Interactables/BP_SequencePuzzlePieces Object Reference"))
  (locals (TempSubObject :type "/Game/TrickPhotography/Programmers/Interactables/BP_SequencePuzzlePieces Object Reference") (bFailedSequence :type Boolean))
  (bind _attemptedsequenceinteractables (`self.AttemptedSequenceInteractables`))
  (bind _sequencedinteractables (`self.SequencedInteractables`))
  (if (`self.bPuzzleCompleted`)
    (`KismetSystemLibrary.PrintString` "Puzzle Already completed no actions have effect")
    (else
      (`/Engine/EditorBlueprintResources/StandardMacros.IsValid` SubObjectedInteracted
        (:`Is Valid`
          (set `local.TempSubObject` SubObjectedInteracted)
          (if (`self.bResetInstantlyOnFail`)
            (if (`self.bObjectActivatedProperly`)
              (for _array_element (`self.SequencedInteractables`)
                (if (`/Game/TrickPhotography/Programmers/Interactables/BP_SequencePuzzlePieces.bObjectActivatedProperly` _array_element)
                  _
                  (elif (== _array_element (`local.TempSubObject`))
                    (`/Game/TrickPhotography/Programmers/Interactables/BP_SequencePuzzlePieces.UpdateActivatedStatus` (`local.TempSubObject`) false true)
                    (break)
                    (else
                      (set `local.bFailedSequence` true)
                      (break)))))
              (if (`local.bFailedSequence`)
                ; Failed sequence
                (`self.UpdateActivatedStatus` true :!label _label)
                (for _array_element_2 (`self.SequencedInteractables`)
                  (`/Game/TrickPhotography/Programmers/Interactables/BP_SequencePuzzlePieces.UpdateActivatedStatus` _array_element_2 true false))
                (`KismetArrayLibrary.Array_Clear` (`self.AttemptedSequenceInteractables`))
                (elif (`/Game/TrickPhotography/Programmers/Interactables/BP_SequencePuzzlePieces.bObjectActivatedProperly` (`|GetArrayItem` _sequencedinteractables (`KismetArrayLibrary.Array_LastIndex` _sequencedinteractables)))
                  (set `self.bPuzzleCompleted` true)
                  (`self.Activate`)))
              (else
                (goto _label)))
            (else
              (`KismetArrayLibrary.Array_AddUnique` _attemptedsequenceinteractables (`local.TempSubObject`))
              (`/Game/TrickPhotography/Programmers/Interactables/BP_SequencePuzzlePieces.UpdateActivatedStatus` (`local.TempSubObject`) false true)
              (if (== (`KismetArrayLibrary.Array_Length` _attemptedsequenceinteractables) (`KismetArrayLibrary.Array_Length` (`self.SequencedInteractsIncludingSelf`))) :!label _label_2
                (for (_array_element_3 _array_index) (`self.SequencedInteractsIncludingSelf`)
                  (if (not (== _array_element_3 (`|GetArrayItem` (`self.AttemptedSequenceInteractables`) _array_index)))
                    (set `local.bFailedSequence` true)
                    (goto _label)))
                (if (not (`local.bFailedSequence`))
                  (set `self.bPuzzleCompleted` true)
                  (`self.Activate`)
                  (`KismetArrayLibrary.Array_Clear` (`self.AttemptedSequenceInteractables`)))))))
        (:`Is Not Valid`
          (if (not (`self.bResetInstantlyOnFail`))
            (`KismetArrayLibrary.Array_AddUnique` (`self.AttemptedSequenceInteractables`) self)
            (goto _label_2)))))))

(fn `SetMaterial`
  (params (Mat :type "MaterialInstance Object Reference"))
  (`PrimitiveComponent.SetMaterial` (`self.FilterStaticMesh`) 0 Mat)
  (`FilterStaticMeshComponent.SetMainMaterial` (`self.FilterStaticMesh`) Mat))

(fn `UserConstructionScript`
  (`parent.UserConstructionScript`))