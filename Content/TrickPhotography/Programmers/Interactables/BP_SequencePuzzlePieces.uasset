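; An interactable piece of a sequence puzzle that highlights on hover and reports non-Cammy interactions to its main puzzle object while not yet correctly activated.
; UpdateActivatedStatus swaps the idol material between plain and glowing, and activates or deactivates linked objects through BPI_Activatable, toggling visibility for those without the interface.
; On failure, a delayable loop flashes the glow before resetting the piece, without touching linked objects.
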(event `self.ReceiveBeginPlay`
  (`self.UpdateActivatedStatus` false))

(event `/Game/TrickPhotography/Programmers/Core/Interfaces/BPI_Interactable.InteractStart`
  (params (HeldItem :type "PickupableInterface Interface") (bIsCammy :type Boolean) (HitComponent :type "PrimitiveComponent Object Reference"))
  (bind _puzzlemainobject (`self.PuzzleMainObject`))
  (if bIsCammy
    _
    (elif (not (`self.bObjectActivatedProperly`))
      (`/Engine/EditorBlueprintResources/StandardMacros.IsValid` _puzzlemainobject
        (:`Is Valid`
          (`/Game/TrickPhotography/Programmers/Interactables/BP_SequencePuzzleStart.ObjectInteractedWith` _puzzlemainobject self))))))

(event `UpdateActivatedStatus`
  (params (bFailed :type Boolean) (bSetActivated :type Boolean))
  (if bFailed
    (`/Game/TrickPhotography/Programmers/Core/BaseClasses/CustomMacros.DelayableForLoop` 0 5 :!label _label
      (:`LoopBody`
        (`self.SetMaterial` "/Game/TrickPhotography/Art/Materials/Idols/M_Idol2.M_Idol2")
        (`KismetSystemLibrary.Delay` 0.2)
        (`self.SetMaterial` "/Game/TrickPhotography/Art/Materials/Idols/M_Idol2Glow.M_Idol2Glow")
        (`KismetSystemLibrary.Delay` 0.1)
        (goto _label :!via `CountUp`))
      (:`Completed`
        (`self.SetMaterial` "/Game/TrickPhotography/Art/Materials/Idols/M_Idol2.M_Idol2")
        (set `self.bObjectActivatedProperly` false)))
    (else
      (bind _output_get (set `self.bObjectActivatedProperly` bSetActivated))
      (if _output_get
        (`self.SetMaterial` "/Game/TrickPhotography/Art/Materials/Idols/M_Idol2Glow.M_Idol2Glow")
        (for _array_element (`self.ObjectsToActivateWhenActivated`)
          (bind _asbpi_activatable (cast `/Game/TrickPhotography/Programmers/Core/Interfaces/BPI_Activatable` _array_element)
            (:`then`
              (`/Game/TrickPhotography/Programmers/Core/Interfaces/BPI_Activatable.Activate` _asbpi_activatable))
            (:`CastFailed`
              (`self.SetActorHiddenInGame` _array_element false))))
        (else
          (`self.SetMaterial` "/Game/TrickPhotography/Art/Materials/Idols/M_Idol2.M_Idol2")
          (for _array_element_2 (`self.ObjectsToActivateWhenActivated`)
            (bind _asbpi_activatable_2 (cast `/Game/TrickPhotography/Programmers/Core/Interfaces/BPI_Activatable` _array_element_2)
              (:`then`
                (`/Game/TrickPhotography/Programmers/Core/Interfaces/BPI_Activatable.Deactivate` _asbpi_activatable_2))
              (:`CastFailed`
                (`self.SetActorHiddenInGame` _array_element_2 true)))))))))

(event `/Game/TrickPhotography/Programmers/Core/Interfaces/BPI_Interactable.HoverEnd`
  (params (HeldItem :type "PickupableInterface Interface"))
  (`self.SetPPMHighlight` "None"))

(fn `HoverOngoing`
  (params (HeldItem :type "PickupableInterface Interface") (HitComponent :type "PrimitiveComponent Object Reference"))
  (returns (bIsInteractable :type Boolean))
  (return false))

(fn `HoverStart`
  (params (HeldItem :type "PickupableInterface Interface") (HitComponent :type "PrimitiveComponent Object Reference"))
  (returns (bIsInteractable :type Boolean))
  (`self.SetPPMHighlight` "HighlightPickup")
  (return false))

(fn `SetMaterial`
  (params (Mat :type "MaterialInstance Object Reference"))
  (`PrimitiveComponent.SetMaterial` (`self.FilterStaticMesh`) 0 Mat)
  (`FilterStaticMeshComponent.SetMainMaterial` (`self.FilterStaticMesh`) Mat))

(fn `UserConstructionScript`)