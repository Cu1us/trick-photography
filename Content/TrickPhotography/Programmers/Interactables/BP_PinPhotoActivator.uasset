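; Interactable pin spot that activates when a photo is pinned to it, optionally requiring a particular photo (by variable name, a thermal shot of a lit fireplace).
; It records its static mesh's location and rotation as the placement transform on BeginPlay.
; With the requirement on, a trigger volume tells the main character to look for the target actor class while inside.
; Pinned photos with the wrong filter or subject are then destroyed.
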(event `self.ReceiveBeginPlay`
  (bind (_returnvalue_location _returnvalue_rotation) (`KismetMathLibrary.BreakTransform` (`SceneComponent.K2_GetComponentToWorld` (`self.StaticMesh`))))
  (`parent.ReceiveBeginPlay`)
  (set `self.PlacePos` (`KismetMathLibrary.MakeTransform` _returnvalue_location _returnvalue_rotation)))

(event `self.ReceiveActorBeginOverlap`
  (params (OtherActor :type "Actor Object Reference")))

(event `PhotoPinned`
  (params (PhotoPinned :type "/Game/TrickPhotography/Programmers/Core/Camera/BP_Photograph Object Reference"))
  (if (`self.bRequireLitFireplaceThermal`)
    (if (`|EnumEquality` (`/Game/TrickPhotography/Programmers/Core/Camera/BP_Photograph.FilterType` PhotoPinned) "NewEnumerator1")
      (if (== (`/Game/TrickPhotography/Programmers/Core/Camera/BP_Photograph.ClassInPhoto` PhotoPinned) (`self.ActorToLookFor`))
        (`self.Activate` :!label _label)
        (else
          (`self.K2_DestroyActor` PhotoPinned :!label _label_2)))
      (else
        (goto _label_2)))
    (else
      (goto _label))))

(event `self.IfRequireSpecialAndPlayerInThisCheckForActorInPhoto.OnComponentBeginOverlap`
  (params (OverlappedComponent :type "PrimitiveComponent Object Reference") (OtherActor :type "Actor Object Reference") (OtherComp :type "PrimitiveComponent Object Reference") (OtherBodyIndex :type Integer) (bFromSweep :type Boolean) (SweepResult :type "HitResult Structure (by ref)"))
  (if (`self.bRequireLitFireplaceThermal`)
    (bind _asbp_main_character (cast `/Game/TrickPhotography/Programmers/Core/Player/BP_MainCharacter` OtherActor))
    (`/Game/TrickPhotography/Programmers/Core/Player/BP_MainCharacter.InAreaOfSpecificPhotoObjects` _asbp_main_character (`self.ActorToLookFor`) true)))

(event `self.IfRequireSpecialAndPlayerInThisCheckForActorInPhoto.OnComponentEndOverlap`
  (params (OverlappedComponent :type "PrimitiveComponent Object Reference") (OtherActor :type "Actor Object Reference") (OtherComp :type "PrimitiveComponent Object Reference") (OtherBodyIndex :type Integer))
  (if (`self.bRequireLitFireplaceThermal`)
    (bind _asbp_main_character (cast `/Game/TrickPhotography/Programmers/Core/Player/BP_MainCharacter` OtherActor))
    (`/Game/TrickPhotography/Programmers/Core/Player/BP_MainCharacter.InAreaOfSpecificPhotoObjects` _asbp_main_character null false)))

(fn `UserConstructionScript`
  (`parent.UserConstructionScript`))