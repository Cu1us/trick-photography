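; Door actor for statue puzzles that swings around its yaw axis when activated.
; On BeginPlay it calls the parent logic and caches its starting yaw.
; The Activate event prints a debug string and plays a Timeline that adds its animated offset to that yaw, keeping roll and pitch unchanged.
; No closing or deactivation logic is defined here.
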(event `self.ReceiveBeginPlay`
  (bind (_returnvalue_roll _returnvalue_pitch _returnvalue_yaw) (`KismetMathLibrary.BreakRotator` (`self.K2_GetActorRotation`)))
  (`parent.ReceiveBeginPlay`)
  (set `self.InitialRot` _returnvalue_yaw))

(event `/Game/TrickPhotography/Programmers/Core/Interfaces/BPI_Activatable.Activate`
  (bind (_returnvalue_roll _returnvalue_pitch) (`KismetMathLibrary.BreakRotator` (`self.K2_GetActorRotation`)))
  (`KismetSystemLibrary.PrintString` "Activated")
  (bind (_direction _z) (`Timeline|Timeline`)
    (:`Update`
      (`self.K2_SetActorRotation` (`KismetMathLibrary.MakeRotator` _returnvalue_roll _returnvalue_pitch (+ _z (`self.InitialRot`)))))))

(fn `UserConstructionScript`
  (`parent.UserConstructionScript`))