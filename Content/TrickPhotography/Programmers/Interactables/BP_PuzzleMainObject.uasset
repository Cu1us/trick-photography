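; Main object of an ordered-interaction puzzle, an idol that glows when lit and calls Activate once the sequence is solved.
; It registers itself with its SequencedInteractables, whose interactions are validated in ObjectInteractedWith.
; With ResetInstantlyOnFail, the main object must be lit first and each sub-object is checked immediately.
; Otherwise attempts, including itself, are compared once all are recorded, and a failed sequence unlights everything.
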(event `self.ReceiveBeginPlay`
  (bind _sequencedinteractsincludingself (`self.SequencedInteractsIncludingSelf`))
  (`parent.ReceiveBeginPlay`)
  (for _array_element (`self.SequencedInteractables`)
    (set `/Game/TrickPhotography/Programmers/Interactables/BP_PuzzleSubObject.PuzzleMainObject` self _array_element))
  (`KismetArrayLibrary.Array_Add` _sequencedinteractsincludingself self)
  (`KismetArrayLibrary.Array_Append` _sequencedinteractsincludingself (`self.SequencedInteractables`)))

(event `/Game/TrickPhotography/Programmers/Core/Interfaces/BPI_Interactable.InteractStart`
  (params (HeldItem :type "PickupableInterface Interface") (bIsCammy :type Boolean) (HitComponent :type "PrimitiveComponent Object Reference"))
  (if (`self.bPuzzleCompleted`)
    (`KismetSystemLibrary.PrintString` "Already completed")
    (else
      (`self.UpdateActivatedStatus` true))))

(event `UpdateActivatedStatus`
  (params (bSetActivated :type Boolean))
  (bind _output_get (set `self.bObjectActivatedProperly` bSetActivated))
  (if _output_get
    (`PrimitiveComponent.SetMaterial` (`self.FilterStaticMesh`) 0 "/Game/TrickPhotography/Art/Materials/Idols/M_Idol1glow.M_Idol1glow")
    (if (not (`self.bResetInstantlyOnFail`))
      (`self.ObjectInteractedWith` null))
    (else
      (`PrimitiveComponent.SetMaterial` (`self.FilterStaticMesh`) 0 "/Game/TrickPhotography/Art/Materials/Idols/M_Idol1.M_Idol1"))))

(fn `Activate`
  (`parent.Activate`))

(fn `HoverOngoing`
  (params (HeldItem :type "PickupableInterface Interface") (HitComponent :type "PrimitiveComponent Object Reference"))
  (returns (bIsInteractable :type Boolean))
  (return false))

(fn `HoverStart`
  (params (HeldItem :type "PickupableInterface Interface") (HitComponent :type "PrimitiveComponent Object Reference"))
  (returns (bIsInteractable :type Boolean))
  (return false))

(fn `ObjectInteractedWith`
  (params (SubObjectedInteracted :type "/Game/TrickPhotography/Programmers/Interactables/BP_PuzzleSubObject Object Reference"))
  (locals (TempSubObject :type "/Game/TrickPhotography/Programmers/Interactables/BP_PuzzleSubObject Object Reference") (bFailedSequence :type Boolean))
  (bind _attemptedsequenceinteractables (`self.AttemptedSequenceInteractables`))
  (bind _sequencedinteractables (`self.SequencedInteractables`))
  (if (`self.bPuzzleCompleted`)
    (`KismetSystemLibrary.PrintString` "Puzzle Already completed no actions have effect")
    (else
      (`/Engine/EditorBlueprintResources/StandardMacros.IsValid` SubObjectedInteracted
        (:`Is Valid`
          (set `local.TempSubObject` SubObjectedInteracted)
          (if (`self.bResetInstantlyOnFail`)
            (if (`self.bObjectActivatedProperly`)
              (for _array_element (`self.SequencedInteractables`)
                (if (`/Game/TrickPhotography/Programmers/Interactables/BP_PuzzleSubObject.bObjectActivatedProperly` _array_element)
                  _
                  (elif (== _array_element (`local.TempSubObject`))
                    (`/Game/TrickPhotography/Programmers/Interactables/BP_PuzzleSubObject.UpdateActivatedStatus` (`local.TempSubObject`) true)
                    (break)
                    (else
                      (set `local.bFailedSequence` true)
                      (break)))))
              (if (`local.bFailedSequence`)
                ; Failed sequence
                (`self.UpdateActivatedStatus` false :!label _label)
                (for _array_element_2 (`self.SequencedInteractables`)
                  (`/Game/TrickPhotography/Programmers/Interactables/BP_PuzzleSubObject.UpdateActivatedStatus` _array_element_2 false))
                (`KismetArrayLibrary.Array_Clear` (`self.AttemptedSequenceInteractables`))
                (elif (`/Game/TrickPhotography/Programmers/Interactables/BP_PuzzleSubObject.bObjectActivatedProperly` (`|GetArrayItem` _sequencedinteractables (`KismetArrayLibrary.Array_LastIndex` _sequencedinteractables)))
                  (set `self.bPuzzleCompleted` true)
                  (`self.Activate`)))
              (else
                (goto _label)))
            (else
              (`KismetArrayLibrary.Array_AddUnique` _attemptedsequenceinteractables (`local.TempSubObject`))
              (`/Game/TrickPhotography/Programmers/Interactables/BP_PuzzleSubObject.UpdateActivatedStatus` (`local.TempSubObject`) true)
              (if (== (`KismetArrayLibrary.Array_Length` _attemptedsequenceinteractables) (`KismetArrayLibrary.Array_Length` (`self.SequencedInteractsIncludingSelf`))) :!label _label_2
                (for (_array_element_3 _array_index) (`self.SequencedInteractsIncludingSelf`)
                  (if (not (== _array_element_3 (`|GetArrayItem` (`self.AttemptedSequenceInteractables`) _array_index)))
                    (set `local.bFailedSequence` true)))
                (if (`local.bFailedSequence`)
                  (goto _label)
                  (else
                    (set `self.bPuzzleCompleted` true)
                    (`self.Activate`)
                    (`KismetArrayLibrary.Array_Clear` (`self.AttemptedSequenceInteractables`))))))))
        (:`Is Not Valid`
          (if (not (`self.bResetInstantlyOnFail`))
            (`KismetArrayLibrary.Array_AddUnique` (`self.AttemptedSequenceInteractables`) self)
            (goto _label_2)))))))

(fn `UserConstructionScript`
  (`parent.UserConstructionScript`))