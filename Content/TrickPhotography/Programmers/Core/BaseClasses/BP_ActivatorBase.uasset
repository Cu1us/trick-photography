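; BP_ActivatorBase is a base class for activators that hold an on/off IsActivated state and announce changes through dispatchers.
; Activate sets the state and fires OnActivated, and SetActivated routes a boolean to Activate or Deactivate.
; Deactivate is empty as wired: its state reset and OnDeactivated call are disconnected, so this class never switches back off.
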(fn `Activate`
  (set `self.bIsActivated` true)
  (`self.OnActivated`))

(fn `Deactivate`)

(fn `IsActivated`
  (returns (Activated :type Boolean))
  (return (`self.bIsActivated`)))

(fn `SetActivated`
  (params (Activated :type Boolean))
  (if Activated
    (`self.Activate`)
    (else
      (`self.Deactivate`))))

(fn `UserConstructionScript`
  (`parent.UserConstructionScript`))