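; Base actor that lets objects respond to special camera photos such as X-ray, UV and thermal.
; On BeginPlay it caches every component implementing the Filterable interface.
; Each photo start and finish event, including the generic any-photo pair, relays the matching interface message to those components through a shared ForeachFilterableComponent loop.
; The actor itself only dispatches, leaving the response to each component.
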(event `self.ReceiveBeginPlay`
  (set `self.FilterableComponents` (`self.GetComponentsByInterface` "/Script/trickphotography.FilterableInterface")))

(event `FilterableInterface.OnXrayPhotoFinished`
  (bind _array_element (`self.Foreach filterable component`))
  (message `FilterableInterface.OnXrayPhotoFinished` _array_element))

(event `FilterableInterface.OnXrayPhoto`
  (bind _array_element (`self.Foreach filterable component`))
  (message `FilterableInterface.OnXrayPhoto` _array_element))

(event `FilterableInterface.OnUVPhotoFinished`
  (bind _array_element (`self.Foreach filterable component`))
  (message `FilterableInterface.OnUVPhotoFinished` _array_element))

(event `FilterableInterface.OnUVPhoto`
  (bind _array_element (`self.Foreach filterable component`))
  (message `FilterableInterface.OnUVPhoto` _array_element))

(event `FilterableInterface.OnThermalPhotoFinished`
  (bind _array_element (`self.Foreach filterable component`))
  (message `FilterableInterface.OnThermalPhotoFinished` _array_element))

(event `FilterableInterface.OnThermalPhoto`
  (bind _array_element (`self.Foreach filterable component`))
  (message `FilterableInterface.OnThermalPhoto` _array_element))

(event `FilterableInterface.OnAnyPhotoFinished`
  (bind _array_element (`self.Foreach filterable component`))
  (message `FilterableInterface.OnAnyPhotoFinished` _array_element))

(event `FilterableInterface.OnAnyPhoto`
  (bind _array_element (`self.Foreach filterable component`))
  (message `FilterableInterface.OnAnyPhoto` _array_element))

(fn `UserConstructionScript`)