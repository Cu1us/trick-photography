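; Static mesh component base class that changes its appearance for thermal, UV and X-ray photos in a photography game.
; For each photo type, an interaction setting either swaps material slot 0 to that filter's material or hides the mesh and flags it.
; When any photo finishes, it restores the default material cached at BeginPlay and re-shows the mesh if the hidden flag is set, which is never cleared.
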(event `self.ReceiveBeginPlay`
  (set `self.DefaultMaterial` (`self.GetMaterial` 0)))

(event `FilterableInterface.OnAnyPhotoFinished`
  (`self.SetMaterial` 0 (`self.DefaultMaterial`))
  (if (`self.bHiddenDueToFilterChange`)
    (`self.SetVisibility` true)))

(event `FilterableInterface.OnThermalPhoto`
  (switch `FilterVisibility` (`self.ThermalInteraction`)
    (:`Visible`
      (`self.SetMaterial` 0 (`self.ThermalMaterial`)))
    (:`Hidden`
      (`self.SetVisibility` false)
      (set `self.bHiddenDueToFilterChange` true))))

(event `FilterableInterface.OnUVPhoto`
  (switch `FilterVisibility` (`self.UVInteraction`)
    (:`Visible`
      (`self.SetMaterial` 0 (`self.UVMaterial`)))
    (:`Hidden`
      (`self.SetVisibility` false)
      (set `self.bHiddenDueToFilterChange` true))))

(event `FilterableInterface.OnXrayPhoto`
  (switch `FilterVisibility` (`self.XrayInteraction`)
    (:`Visible`
      (`self.SetMaterial` 0 (`self.XrayMaterial`)))
    (:`Hidden`
      (`self.SetVisibility` false)
      (set `self.bHiddenDueToFilterChange` true))))