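; BP_FilterableSpotLight is a spot light whose visibility changes with the photo filter being captured.
; Photo events for thermal, UV, X-ray and invisibility shots set the light component's visibility from a matching per-filter flag.
; BeginPlay and the photo-finished event restore the normal player-facing visibility flag.
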(event `self.ReceiveBeginPlay`
  (`SceneComponent.SetVisibility` (`self.SpotLightComponent`) (`self.bVisibleByPlayer`) false :!label _label))

(event `FilterableInterface.OnAnyPhotoFinished`
  (goto _label))

(event `FilterableInterface.OnThermalPhoto`
  (`SceneComponent.SetVisibility` (`self.SpotLightComponent`) (`self.bVisibleInThermal`) false))

(event `FilterableInterface.OnUVPhoto`
  (`SceneComponent.SetVisibility` (`self.SpotLightComponent`) (`self.bVisibleInUV`) false))

(event `FilterableInterface.OnXrayPhoto`
  (`SceneComponent.SetVisibility` (`self.SpotLightComponent`) (`self.bVisibleInXray`) false))

(event `FilterableInterface.OnInvisPhoto`
  (`SceneComponent.SetVisibility` (`self.SpotLightComponent`) (`self.bVisibleInInvis`) false))

(fn `UserConstructionScript`)