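; BP_FilterVisibilityToggler shows or hides a list of affected actors according to the photo filter in use.
; Thermal, UV and X-ray photo events each apply their own visibility flag, and finishing any photo restores the outside-photo flag.
; Visibility is set only on each actor's root component, without propagating to children.
; The normal-photo visibility call is unconnected, so that flag has no effect.
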(event `FilterableInterface.OnAnyPhoto`)

(event `FilterableInterface.OnAnyPhotoFinished`
  (`self.SetVisibilityOfAffected` (`self.bVisibleOutsidePhotos`)))

(event `FilterableInterface.OnThermalPhoto`
  (`self.SetVisibilityOfAffected` (`self.bVisibleInThermal`)))

(event `FilterableInterface.OnUVPhoto`
  (`self.SetVisibilityOfAffected` (`self.bVisibleInUV`)))

(event `FilterableInterface.OnXrayPhoto`
  (`self.SetVisibilityOfAffected` (`self.bVisibleInXray`)))

(fn `SetVisibilityOfAffected`
  (params (Visible :type Boolean))
  (for _array_element (`self.AffectedActors`)
    (`SceneComponent.SetVisibility` (`Actor.RootComponent` _array_element) Visible false)))

(fn `UserConstructionScript`)