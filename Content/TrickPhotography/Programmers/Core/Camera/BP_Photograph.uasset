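; BP_Photograph is a photograph prop that displays a given image on its mesh and can fade that image in.
; SetImage lazily creates a dynamic instance of M_Photograph_Photo on material element 1 and assigns the texture to its Image parameter.
; The FadeIn event plays a timeline whose curve feeds SetFadeAmount, which writes a clamped Opacity to that material instance if it exists.
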(event `FadeIn`
  (bind (_direction _photofadeincurve) (`Timeline|PhotoFadeTimeline`)
    (:`Update`
      (`self.SetFadeAmount` _photofadeincurve))))

(fn `SetFadeAmount`
  (params (ImageOpacity :type "Float (double-precision)"))
  (bind _photomaterialinstance (`self.PhotoMaterialInstance`))
  (`/Engine/EditorBlueprintResources/StandardMacros.IsValid` _photomaterialinstance
    (:`Is Valid`
      (`MaterialInstanceDynamic.SetScalarParameterValue` _photomaterialinstance "Opacity" (`KismetMathLibrary.FClamp` ImageOpacity)))))

(fn `SetImage`
  (params (Image :type "Texture Object Reference"))
  (`/Engine/EditorBlueprintResources/StandardMacros.IsValid` (`self.PhotoMaterialInstance`)
    (:`Is Valid`
      _)
    (:`Is Not Valid`
      (bind _returnvalue (`PrimitiveComponent.CreateDynamicMaterialInstance` (`self.Photograph`) 1 "/Game/TrickPhotography/Art/Enviroment/Materials_MeshSpecific/Photograph/M_Photograph_Photo.M_Photograph_Photo" "None"))
      (set `self.PhotoMaterialInstance` _returnvalue)))
  (`MaterialInstanceDynamic.SetTextureParameterValue` (`self.PhotoMaterialInstance`) "Image" Image))

(fn `UserConstructionScript`)