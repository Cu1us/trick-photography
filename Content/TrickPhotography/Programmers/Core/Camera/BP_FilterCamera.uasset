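; Filter camera actor that takes filtered photos (thermal, UV, X-Ray, Flash) and hands them to Cammy as pickupable photographs.
; CaptureImage briefly sets the GameMode's world filter while a SceneCapture renders to a new render target.
; An overlap check gives imageless photos inside geometry and, while looked through, hides overlapping actors behind a blocking plane.
; BeginPlay pre-warms filter shaders with one capture per tick.
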(event `Key|Y`
  (params (Key :type "Key Structure"))
  ; OLD TESTING SYSTEM
)

(event `self.ReceiveBeginPlay`
  (bind _asmain_player_controller (cast `/Game/TrickPhotography/Programmers/Core/Player/MainPlayerController` (`GameplayStatics.GetPlayerController` 0))
    (:`then`
      (set `self.As Main Player Controller` _asmain_player_controller))
    (:`CastFailed`
      _))
  (`KismetSystemLibrary.DelayUntilNextTick`)
  (`self.CaptureImage` "NewEnumerator1")
  (`KismetSystemLibrary.DelayUntilNextTick`)
  (`self.CaptureImage` "NewEnumerator2")
  (`KismetSystemLibrary.DelayUntilNextTick`)
  (`self.CaptureImage` "NewEnumerator3")
  (`KismetSystemLibrary.DelayUntilNextTick`)
  (`self.CaptureImage` "NewEnumerator4"))

(event `self.ReceiveTick`
  (params (DeltaSeconds :type "Float (single-precision)"))
  (bind _hiddenactors (`self.HiddenActors`))
  (bind _as_main_player_controller (`self.As Main Player Controller`))
  (for _array_element _hiddenactors
    (`self.SetActorHiddenInGame` _array_element false))
  (`KismetArrayLibrary.Array_Clear` _hiddenactors)
  (if (`self.bBeingLookedThrough`)
    (bind _outactors (`KismetSystemLibrary.BoxOverlapActors` (`self.K2_GetActorLocation`) (10.0 10.0 10.0) (`self.Object Types`) null (`|MakeArray` (`/Game/TrickPhotography/Programmers/Core/Player/MainPlayerController.MainChar` _as_main_player_controller) (`/Game/TrickPhotography/Programmers/Core/Player/MainPlayerController.CammyChar` _as_main_player_controller) self :!type "Actor Object Reference")))
    (bind _output_get (set `self.HiddenActors` _outactors))
    (for _array_element_2 _output_get
      (`self.SetActorHiddenInGame` _array_element_2 true))
    (`SceneComponent.SetHiddenInGame` (`self.Plane`) (not (> (`KismetArrayLibrary.Array_Length` _outactors) 0)) false)))

(fn `CaptureImage`
  (params (`Filter Type` :type "/Game/TrickPhotography/Programmers/Enums/FilterType Enum" :default "NewEnumerator0"))
  (returns (`Output Render Target` :type "TextureRenderTarget2D Object Reference"))
  ; Prepare texture for rendering
  (bind _returnvalue (`KismetRenderingLibrary.CreateRenderTarget2D` 512 512))
  (bind _output_get (set `SceneCaptureComponent2D.TextureTarget` _returnvalue (`self.SceneCapture`)))
  (bind _asgm_main_game (cast `/Game/TrickPhotography/Programmers/Core/GM_MainGame` (`GameplayStatics.GetGameMode`)))
  (`/Game/TrickPhotography/Programmers/Core/GM_MainGame.SetWorldFilter` _asgm_main_game `Filter Type`)
  (`SceneCaptureComponent2D.CaptureScene` (`self.SceneCapture`))
  (`/Game/TrickPhotography/Programmers/Core/GM_MainGame.ResetWorldFilter` _asgm_main_game)
  (return _output_get))

(fn `SpawnPhotograph`
  (params (Image :type "TextureRenderTarget2D Object Reference") (Transform :type "Transform Structure"))
  (returns (`New Photograph` :type "/Game/TrickPhotography/Programmers/Core/Camera/BP_Photograph Object Reference"))
  (bind _returnvalue (`|SpawnActorFromClass` "/Game/TrickPhotography/Programmers/Core/Camera/BP_Photograph.BP_Photograph_C" Transform "AlwaysSpawn" "MultiplyWithRoot" null null))
  (`/Game/TrickPhotography/Programmers/Core/Camera/BP_Photograph.SetImage` _returnvalue Image)
  (`/Game/TrickPhotography/Programmers/Core/Camera/BP_Photograph.FadeIn` _returnvalue)
  (bind _asgm_main_game (cast `/Game/TrickPhotography/Programmers/Core/GM_MainGame` (`GameplayStatics.GetGameMode`)))
  (`/Game/TrickPhotography/Programmers/Core/GM_MainGame.RegisterNewFilterable` _asgm_main_game _returnvalue)
  (return _returnvalue))

(fn `TakePhotoAsCammy`
  (params (CammyChar :type "/Game/TrickPhotography/Programmers/Core/Player/BP_CammyCharacter Object Reference") (`Filter Type` :type "/Game/TrickPhotography/Programmers/Enums/FilterType Enum" :default "NewEnumerator0"))
  (bind _outactors (`KismetSystemLibrary.BoxOverlapActors` (`self.K2_GetActorLocation`) (10.0 10.0 10.0) (`self.Object Types`) null (`|MakeArray` CammyChar (`/Game/TrickPhotography/Programmers/Core/Player/BP_CammyCharacter.MainCharacter` CammyChar) :!type "Actor Object Reference")))
  (if (> (`KismetArrayLibrary.Array_Length` _outactors) 0)
    ; Spawn black photo
    (`KismetSystemLibrary.PrintString` "Photo in wall")
    (bind _new_photograph (`self.SpawnPhotograph` null (`KismetMathLibrary.MakeTransform` (0.0 0.0 0.0) (struct) (3.0 3.0 3.0))))
    (bind _aspickupable_interface (cast `PickupableInterface` _new_photograph))
    (`/Game/TrickPhotography/Programmers/Core/Player/BP_CammyCharacter.PhotoToCammy` (`local.CammyChar`) _aspickupable_interface)
    (else
      (switch `/Game/TrickPhotography/Programmers/Enums/FilterType` (`local.Filter Type`)
        (:`NewEnumerator0`
          _)
        (:`NewEnumerator1`
          _)
        (:`NewEnumerator2`
          (`SceneComponent.SetVisibility` (`self.UVSpotLight`) true false))
        (:`NewEnumerator3`
          _)
        (:`NewEnumerator4`
          _)
        (:`NewEnumerator5`
          _))
      (bind _output_render_target (`self.CaptureImage` (`local.Filter Type`)))
      (bind _new_photograph_2 (`self.SpawnPhotograph` _output_render_target (`KismetMathLibrary.MakeTransform` (0.0 0.0 0.0) (struct) (3.0 3.0 3.0))))
      (bind _aspickupable_interface_2 (cast `PickupableInterface` _new_photograph_2))
      (`/Game/TrickPhotography/Programmers/Core/Player/BP_CammyCharacter.PhotoToCammy` (`local.CammyChar`) _aspickupable_interface_2)
      (`SceneComponent.SetVisibility` (`self.UVSpotLight`) false false))))

(fn `UserConstructionScript`)