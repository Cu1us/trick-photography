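; BP_CammyCharacter is Cammy, a controllable camera character that can be held by the main character or placed in the world.
; It starts attached to BP_MainCharacter's hand socket without collision; Place detaches it in front of them and restores collision.
; On controller change it adds its input mapping, moving along the main character's forward and right axes.
; Snap input triggers its child filter camera, and photos can attach to its PhotoEject socket.
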(event `self.ReceiveControllerChanged`
  (params (OldController :type "Controller Object Reference") (NewController :type "Controller Object Reference"))
  (bind _asmain_player_controller (cast `/Game/TrickPhotography/Programmers/Core/Player/MainPlayerController` NewController))
  (`EnhancedInputSubsystemInterface.AddMappingContext` (pcsubsystem `EnhancedInputLocalPlayerSubsystem` _asmain_player_controller) "/Game/TrickPhotography/Programmers/Core/Inputs/IMC_Cammy.IMC_Cammy" 0 (struct)))

(event `EnhancedInput|/Game/TrickPhotography/Programmers/Core/Inputs/IA_Move`
  (params (ActionValue :type "Vector2D Structure") (ElapsedSeconds :type "Float (double-precision)") (TriggeredSeconds :type "Float (double-precision)") (InputAction :type "InputAction Object Reference" :default "/Game/TrickPhotography/Programmers/Core/Inputs/IA_Move.IA_Move"))
  (bind _maincharacter (`self.MainCharacter`))
  (:`Triggered`
    (`self.AddMovementInput` (`self.GetActorRightVector` _maincharacter) ActionValue_X)
    (`self.AddMovementInput` (`self.GetActorForwardVector` _maincharacter) ActionValue_Y)))

(event `self.ReceiveBeginPlay`
  (bind _asmain_player_controller (cast `/Game/TrickPhotography/Programmers/Core/Player/MainPlayerController` (`GameplayStatics.GetPlayerController` 0)))
  (set `self.PlayerController` _asmain_player_controller)
  (bind _returnvalue (`GameplayStatics.GetActorOfClass` "/Game/TrickPhotography/Programmers/Core/Player/BP_MainCharacter.BP_MainCharacter_C"))
  (set `self.MainCharacter` _returnvalue)
  (`self.Recall`))

(event `Recall`
  (`self.K2_AttachToComponent` (`/Game/TrickPhotography/Programmers/Core/Player/BP_MainCharacter.RHand` (`self.MainCharacter`)) "HandSocket" "SnapToTarget" "SnapToTarget" "KeepRelative")
  (`self.SetActorEnableCollision` false))

(event `Place`
  (bind _maincharacter (`self.MainCharacter`))
  (`self.K2_DetachFromActor` "KeepRelative")
  (`self.K2_SetActorLocation` (+ (`self.K2_GetActorLocation` _maincharacter) (* (`self.GetActorForwardVector` _maincharacter) 100.0)))
  (`self.SetActorHiddenInGame` false)
  (`self.SetActorEnableCollision` true))

(event `EnhancedInput|/Game/TrickPhotography/Programmers/Core/Inputs/IA_SnapPhoto`
  (params (ActionValue :type Boolean) (ElapsedSeconds :type "Float (double-precision)") (TriggeredSeconds :type "Float (double-precision)") (InputAction :type "InputAction Object Reference" :default "/Game/TrickPhotography/Programmers/Core/Inputs/IA_SnapPhoto.IA_SnapPhoto"))
  (:`Started`
    (bind _asbp_filter_camera (cast `/Game/TrickPhotography/Programmers/Core/Camera/BP_FilterCamera` (`ChildActorComponent.ChildActor` (`self.BP_Camera_Prototype`))))
    (`/Game/TrickPhotography/Programmers/Core/Camera/BP_FilterCamera.TakePhotoAsCammy` _asbp_filter_camera self "NewEnumerator0")))

(event `AttachPhotoToCammy`
  (params (`New Photo` :type "/Game/TrickPhotography/Programmers/Core/Camera/BP_Photograph Object Reference"))
  (`self.K2_AttachToComponent` `New Photo` (`self.Mesh`) "PhotoEject" "KeepRelative" "KeepRelative" "KeepRelative" false))

(fn `UserConstructionScript`)