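; BP_ActivatableDecal is a decal that shows or hides when its Activator fires activated and deactivated events.
; BeginPlay sets the starting alpha and binds to those events, with InvertVisibility swapping which one shows the decal.
; Transitions either snap or, with AnimateTransition, play the AnimateDecal timeline forward or in reverse.
; SetAlpha writes only the decal color's alpha channel and prints a debug string.
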(event `self.ReceiveBeginPlay`
  (bind _activator (`self.Activator`))
  (`self.SetAlpha` (`KismetMathLibrary.SelectFloat` 1.0 0.0 (`self.bInvertVisibility`)))
  (add `/Game/TrickPhotography/Programmers/Core/BaseClasses/BP_ActivatorBase.OnActivated` _activator (delegate `/Game/TrickPhotography/Programmers/Core/Interfaces/BPI_Activatable.Activate`))
  (add `/Game/TrickPhotography/Programmers/Core/BaseClasses/BP_ActivatorBase.OnDeactivated` _activator (delegate `/Game/TrickPhotography/Programmers/Core/Interfaces/BPI_Activatable.Deactivate`))
  (`KismetSystemLibrary.PrintString` "bound"))

(event `/Game/TrickPhotography/Programmers/Core/Interfaces/BPI_Activatable.Activate`
  (bind _banimatetransition (`self.bAnimateTransition`))
  (if (`self.bInvertVisibility`)
    (if _banimatetransition :!label _label
      (bind (_direction _alpha) (`Timeline|AnimateDecal` :!via `Reverse` :!label _label_2)
        (:`Update`
          (`self.SetAlpha` _alpha)))
      (else
        (`self.SetAlpha` 0.0)))
    (else
      (if _banimatetransition :!label _label_3
        (goto _label_2)
        (else
          (`self.SetAlpha` 1.0))))))

(event `/Game/TrickPhotography/Programmers/Core/Interfaces/BPI_Activatable.Deactivate`
  (if (`self.bInvertVisibility`)
    (goto _label_3)
    (else
      (goto _label))))

(fn `SetAlpha`
  (params (Alpha :type "Float (double-precision)"))
  (bind _decal (`self.Decal`))
  (bind (_decalcolor_r _decalcolor_g _decalcolor_b) (break `LinearColor` (`DecalComponent.DecalColor` _decal)))
  (`DecalComponent.SetDecalColor` _decal (make `LinearColor` _decalcolor_r _decalcolor_g _decalcolor_b Alpha))
  (`KismetSystemLibrary.PrintString` (`KismetStringLibrary.Concat_StrStr` "alpha set to " (`KismetStringLibrary.Conv_DoubleToString` Alpha))))

(fn `UserConstructionScript`)