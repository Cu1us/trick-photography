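; BP_FilterPostProcessVolumes switches post-process effects for thermal, UV and X-ray photo filters.
; Each filter's photo event enables its matching post process, with the thermal one also printing a debug message.
; OnAnyPhoto disables the non-photo and all-photo post processes.
; OnAnyPhotoFinished restores the non-photo look and disables all the others; nothing here enables the all-photo one.
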(event `FilterableInterface.OnAnyPhotoFinished`
  (set `PostProcessComponent.bEnabled` true (`self.NonPhotoPostProcess`))
  (set `PostProcessComponent.bEnabled` false (`self.AllPhotoPostProcess`))
  (set `PostProcessComponent.bEnabled` false (`self.ThermalPostProcess`))
  (set `PostProcessComponent.bEnabled` false (`self.UVPostProcess`))
  (set `PostProcessComponent.bEnabled` false (`self.XrayPostProcess`)))

(event `FilterableInterface.OnThermalPhoto`
  (set `PostProcessComponent.bEnabled` true (`self.ThermalPostProcess`))
  (`KismetSystemLibrary.PrintString` "thermal enabled"))

(event `FilterableInterface.OnUVPhoto`
  (set `PostProcessComponent.bEnabled` true (`self.UVPostProcess`)))

(event `FilterableInterface.OnXrayPhoto`
  (set `PostProcessComponent.bEnabled` true (`self.XrayPostProcess`)))

(event `FilterableInterface.OnAnyPhoto`
  (set `PostProcessComponent.bEnabled` false (`self.NonPhotoPostProcess`))
  (set `PostProcessComponent.bEnabled` false (`self.AllPhotoPostProcess`)))

(fn `UserConstructionScript`)