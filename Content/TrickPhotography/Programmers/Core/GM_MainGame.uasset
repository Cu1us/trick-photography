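; Main game mode that broadcasts photo filter changes (Thermal, UV, X-Ray, Invisibility) to every filterable actor in the world.
; It gathers FilterableInterface actors on BeginPlay and accepts later registrations through RegisterNewFilterable.
; SetWorldFilter stores the active filter and sends each valid actor the matching photo message, followed by a generic any-photo message.
; ResetWorldFilter sends the corresponding finished messages for the stored filter, without clearing it.
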(event `self.ReceiveBeginPlay`
  (bind _outactors (`GameplayStatics.GetAllActorsWithInterface` "/Script/trickphotography.FilterableInterface"))
  (set `self.AllFilterableObjects` _outactors))

(event `RegisterNewFilterable`
  (params (`New Filterable` :type "FilterableInterface Interface"))
  (bind _asactor (cast `Actor` `New Filterable`)
    (:`then`
      (bind _returnvalue (`KismetArrayLibrary.Array_AddUnique` (`self.AllFilterableObjects`) _asactor))
      (`KismetSystemLibrary.PrintString` (`KismetStringLibrary.Conv_IntToString` _returnvalue)))
    (:`CastFailed`
      (`KismetSystemLibrary.PrintString` "New filterable is not an actor"))))

(event `ResetWorldFilter`
  (for _array_element (`self.AllFilterableObjects`)
    (`/Engine/EditorBlueprintResources/StandardMacros.IsValid` _array_element
      (:`Is Valid`
        (switch `/Game/TrickPhotography/Programmers/Enums/FilterType` (`self.ActiveWorldFilter`)
          (:`NewEnumerator0`
            _)
          (:`NewEnumerator1`
            (message `FilterableInterface.OnThermalPhotoFinished` _array_element))
          (:`NewEnumerator2`
            (message `FilterableInterface.OnUVPhotoFinished` _array_element))
          (:`NewEnumerator3`
            (message `FilterableInterface.OnXrayPhotoFinished` _array_element))
          (:`NewEnumerator5`
            (message `FilterableInterface.OnInvisPhotoFinished` _array_element)))
        (message `FilterableInterface.OnAnyPhotoFinished` _array_element)))))

(event `SetWorldFilter`
  (params (FilterType :type "/Game/TrickPhotography/Programmers/Enums/FilterType Enum" :default "NewEnumerator0"))
  (bind _output_get (set `self.ActiveWorldFilter` FilterType))
  (for _array_element (`self.AllFilterableObjects`)
    (`/Engine/EditorBlueprintResources/StandardMacros.IsValid` _array_element
      (:`Is Valid`
        (switch `/Game/TrickPhotography/Programmers/Enums/FilterType` _output_get
          (:`NewEnumerator0`
            _)
          (:`NewEnumerator1`
            (message `FilterableInterface.OnThermalPhoto` _array_element))
          (:`NewEnumerator2`
            (message `FilterableInterface.OnUVPhoto` _array_element))
          (:`NewEnumerator3`
            (message `FilterableInterface.OnXrayPhoto` _array_element))
          (:`NewEnumerator5`
            (message `FilterableInterface.OnInvisPhoto` _array_element)))
        (message `FilterableInterface.OnAnyPhoto` _array_element)))))

(fn `UserConstructionScript`)