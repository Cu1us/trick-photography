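; First-person player character that carries the Cammy camera character in the right hand and photos or pickups in the left.
; Enhanced Input drives moving, aiming and snapping photos, placing Cammy, interacting, and turning vault dials.
; Per-hand state machines gate actions, with alpha-lerped transforms raising and lowering each hand.
; Line traces handle pickup, swapping and wall placement, and a per-tick trace reports interaction state to MainPlayerController alongside hand states.
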(event `self.ReceiveBeginPlay`
  (bind _cammychar (`self.CammyChar`))
  (bind _asmain_player_controller (cast `/Game/TrickPhotography/Programmers/Core/Player/MainPlayerController` (`GameplayStatics.GetPlayerController` 0)))
  (bind _output_get (set `self.PlayerController` _asmain_player_controller))
  (`/Game/TrickPhotography/Programmers/Core/Player/MainPlayerController.SetCameraViewpoint` _output_get self)
  (bind _returnvalue (`GameplayStatics.GetActorOfClass` "/Game/TrickPhotography/Programmers/Core/Player/BP_CammyCharacter.BP_CammyCharacter_C"))
  (`/Engine/EditorBlueprintResources/StandardMacros.IsValid` _returnvalue
    (:`Is Valid`
      (bind _output_get_2 (set `self.CammyChar` _returnvalue))
      (`/Game/TrickPhotography/Programmers/Core/Player/BP_CammyCharacter.InitializeCammy` _output_get_2 self (`self.PlayerController`))
      (`/Game/TrickPhotography/Programmers/Core/Player/MainPlayerController.InitializeController` (`self.PlayerController`) self _cammychar)
      (bind _asbp_filter_camera (cast `/Game/TrickPhotography/Programmers/Core/Camera/BP_FilterCamera` (`ChildActorComponent.ChildActor` (`/Game/TrickPhotography/Programmers/Core/Player/BP_CammyCharacter.BP_Camera_Prototype` _cammychar))))
      (set `self.Camera` _asbp_filter_camera))
    (:`Is Not Valid`
      (`KismetSystemLibrary.PrintString` "unable to find cammy. game broken"))))

(event `self.ReceiveControllerChanged`
  (params (OldController :type "Controller Object Reference") (NewController :type "Controller Object Reference"))
  (bind _asmain_player_controller (cast `/Game/TrickPhotography/Programmers/Core/Player/MainPlayerController` NewController))
  (`EnhancedInputSubsystemInterface.AddMappingContext` (pcsubsystem `EnhancedInputLocalPlayerSubsystem` _asmain_player_controller) "/Game/TrickPhotography/Programmers/Core/Inputs/IMC_Default.IMC_Default" 0 (struct)))

(event `self.ReceiveTick`
  (params (DeltaSeconds :type "Float (single-precision)"))
  (bind _lookingatinteract (`self.LookingAtInteract`))
  (bind _lookingatinteract_2 (`self.LookingAtInteract`))
  (bind _firstpersoncamera (`self.FirstPersonCamera`))
  (bind _lookingatinteract_3 (`self.LookingAtInteract`))
  (bind _returnvalue (`SceneComponent.K2_GetComponentLocation` _firstpersoncamera))
  (set `self.Delta Seconds` DeltaSeconds)
  (`|ExecutionSequence`
    (:`then_0`
      (switch `/Game/TrickPhotography/Programmers/Enums/ERHandState` (`self.RHandState`)
        (:`NewEnumerator1`
          _)
        (:`NewEnumerator2`
          _))
      (if (<= (`self.RHandLerpAlpha`) 1.0)
        (bind _output_get (set `self.RHandLerpAlpha` (`KismetMathLibrary.FClamp` (+ (* (`self.Delta Seconds`) 2.0) (`self.RHandLerpAlpha`)))))
        (`SceneComponent.K2_SetRelativeTransform` (`self.RHand`) (`KismetMathLibrary.TLerp` (`self.RHandLookTransform`) (`self.RHandRestTransform`) _output_get) false false)
        (if (>= (`self.RHandLerpAlpha`) 1.0)
          (switch `/Game/TrickPhotography/Programmers/Enums/ERHandState` (`self.RHandState`)
            (:`NewEnumerator1`
              (`self.RHandStateChange` "NewEnumerator1"
                (:`ExecOut`
                  _)))
            (:`NewEnumerator2`
              (`self.RHandStateChange` "NewEnumerator2"
                (:`ExecOut`
                  _))))
          (`self.SetCammyRotVis`))))
    (:`then_1`
      (switch `/Game/TrickPhotography/Programmers/Enums/ELHandState` (`self.LHandState`)
        (:`NewEnumerator1`
          _)
        (:`NewEnumerator2`
          _))
      (if (<= (`self.LHandLerpAlpha`) 1.0)
        (bind _output_get_2 (set `self.LHandLerpAlpha` (`KismetMathLibrary.FClamp` (+ (* (`self.Delta Seconds`) 2.0) (`self.LHandLerpAlpha`)))))
        (`SceneComponent.K2_SetRelativeTransform` (`self.LHand`) (`KismetMathLibrary.TLerp` (`self.LHandLookTransform`) (`self.LHandRestTransform`) _output_get_2) false false)
        (if (>= (`self.LHandLerpAlpha`) 1.0)
          (`/Engine/EditorBlueprintResources/StandardMacros.IsValid` (`self.HeldObject`)
            (:`Is Valid`
              (`self.LHandStateChange` "NewEnumerator1"))
            (:`Is Not Valid`
              (`self.LHandStateChange` "NewEnumerator2"))))))
    (:`then_2`
      (switch `/Game/TrickPhotography/Programmers/Enums/ELHandState` (`self.LHandState`)
        (:`NewEnumerator0`
          (if (`KismetSystemLibrary.IsValidInterface` _lookingatinteract_3) :!label _label
            (`/Game/TrickPhotography/Programmers/Core/Interfaces/BPI_Interactable.InteractEnd` _lookingatinteract_3 false)
            (set `self.LookingAtInteract` null)))
        (:`NewEnumerator1`
          (switch `/Game/TrickPhotography/Programmers/Enums/ERHandState` (`self.RHandState`) :!label _label_2
            (:`NewEnumerator0`
              (goto _label))
            (:`NewEnumerator1`
              _)
            (:`NewEnumerator2`
              _)
            (:`NewEnumerator3`
              (goto _label)))
          (if (`/Game/TrickPhotography/Programmers/Core/Player/MainPlayerController.bCammyPossessed` (`self.PlayerController`))
            (`self.InteractionStateChange` "NewEnumerator0")
            (else
              (bind (_outhit _returnvalue_2) (`KismetSystemLibrary.LineTraceSingle` _returnvalue (+ _returnvalue (* (`KismetMathLibrary.GetForwardVector` (`SceneComponent.K2_GetComponentRotation` _firstpersoncamera)) (`self.InteractRange`))) "TraceTypeQuery1" true (`|MakeArray` (`self.CammyChar`) (`self.Camera`) :!type "Actor Object Reference") "ForOneFrame"))
              (if _returnvalue_2
                (bind _asbpi_interactable (cast `/Game/TrickPhotography/Programmers/Core/Interfaces/BPI_Interactable` (`.HitActor` (`GameplayStatics.BreakHitResult` _outhit)))
                  (:`then`
                    (bind _asbp_vault (cast `/Game/TrickPhotography/Programmers/Puzzles/BP_Vault` _asbpi_interactable)
                      (:`then`
                        (if (`KismetSystemLibrary.IsValidInterface` _lookingatinteract_2)
                          (if (not (== _asbp_vault _lookingatinteract_2))
                            (bind _output_get_3 (set `self.LookingAtInteract` _asbp_vault :!label _label_3))
                            (`/Game/TrickPhotography/Programmers/Core/Interfaces/BPI_Interactable.InteractStart` _output_get_3 null false)
                            (`self.InteractionStateChange` "NewEnumerator5"))
                          (else
                            (goto _label_3))))
                      (:`CastFailed`
                        (`self.InteractionStateChange` "NewEnumerator2"))))
                  (:`CastFailed`
                    (cast `PickupableInterface` (`.HitActor` (`GameplayStatics.BreakHitResult` _outhit))
                      (:`then`
                        (if (`KismetSystemLibrary.IsValidInterface` (`self.CurrentPickup`))
                          (`self.InteractionStateChange` "NewEnumerator4")
                          (else
                            (`self.InteractionStateChange` "NewEnumerator3"))))
                      (:`CastFailed`
                        (cast `/Game/TrickPhotography/Programmers/Core/Player/BP_CammyCharacter` (`.HitActor` (`GameplayStatics.BreakHitResult` _outhit))
                          (:`then`
                            (`self.InteractionStateChange` "NewEnumerator3"))
                          (:`CastFailed`
                            (cast `StaticMeshActor` (`.HitActor` (`GameplayStatics.BreakHitResult` _outhit))
                              (:`then`
                                (cast `/Game/TrickPhotography/Programmers/Core/Camera/BP_Photograph` (`self.HeldObject`)
                                  (:`then`
                                    (`self.InteractionStateChange` "NewEnumerator1"))
                                  (:`CastFailed`
                                    (`self.InteractionStateChange` "NewEnumerator2" :!label _label_4
                                      (:`ExecOut`
                                        (if (`KismetSystemLibrary.IsValidInterface` _lookingatinteract)
                                          (`/Game/TrickPhotography/Programmers/Core/Interfaces/BPI_Interactable.InteractEnd` _lookingatinteract false)
                                          (set `self.LookingAtInteract` null)))))))
                              (:`CastFailed`
                                (goto _label_4)))))))))
                (else
                  (goto _label_4))))))
        (:`NewEnumerator2`
          (goto _label_2))
        (:`NewEnumerator3`
          (goto _label))))))

(event `EnhancedInput|/Game/TrickPhotography/Programmers/Core/Inputs/IA_Move`
  (params (ActionValue :type "Vector2D Structure") (ElapsedSeconds :type "Float (double-precision)") (TriggeredSeconds :type "Float (double-precision)") (InputAction :type "InputAction Object Reference" :default "/Game/TrickPhotography/Programmers/Core/Inputs/IA_Move.IA_Move"))
  (:`Triggered`
    (`/Game/TrickPhotography/Programmers/Core/Player/MainPlayerController.RefreshInputDevice` (`self.PlayerController`))
    (`self.AddMovementInput` (`self.GetActorRightVector`) ActionValue_X)
    (`self.AddMovementInput` (`self.GetActorForwardVector`) ActionValue_Y)))

(event `EnhancedInput|/Game/TrickPhotography/Programmers/Core/Inputs/IA_Look`
  (params (ActionValue :type "Vector2D Structure") (ElapsedSeconds :type "Float (double-precision)") (TriggeredSeconds :type "Float (double-precision)") (InputAction :type "InputAction Object Reference" :default "/Game/TrickPhotography/Programmers/Core/Inputs/IA_Look.IA_Look"))
  (bind (_returnvalue_x _returnvalue_y) (`KismetMathLibrary.BreakVector2D` (* ActionValue 50.0)))
  (bind (_relativerotation_roll _relativerotation_pitch) (`KismetMathLibrary.BreakRotator` (`SceneComponent.RelativeRotation` (`self.FirstPersonCamera`))))
  (:`Triggered`
    (`/Game/TrickPhotography/Programmers/Core/Player/MainPlayerController.RefreshInputDevice` (`self.PlayerController`))
    (`self.AddControllerYawInput` _returnvalue_x)
    (`SceneComponent.K2_SetRelativeRotation` (`self.FirstPersonCamera`) (`KismetMathLibrary.MakeRotator` 0.0 (`KismetMathLibrary.ClampAngle` (+ (* _returnvalue_y 2.0) _relativerotation_pitch) -80.0 80.0)) false false)))

(event `EnhancedInput|/Game/TrickPhotography/Programmers/Core/Inputs/IA_LookAtPhoto`
  (params (ActionValue :type Boolean) (ElapsedSeconds :type "Float (double-precision)") (TriggeredSeconds :type "Float (double-precision)") (InputAction :type "InputAction Object Reference" :default "/Game/TrickPhotography/Programmers/Core/Inputs/IA_LookAtPhoto.IA_LookAtPhoto"))
  (:`Triggered`
    (switch `/Game/TrickPhotography/Programmers/Enums/ERHandState` (`self.RHandState`)
      (:`NewEnumerator1`
        _)
      (:`NewEnumerator2`
        _))
    (switch `/Game/TrickPhotography/Programmers/Enums/ELHandState` (`self.LHandState`)
      (:`NewEnumerator1`
        (`self.LHandStateChange` "NewEnumerator3"
          (:`ExecOut`
            _)))
      (:`NewEnumerator3`
        _))
    (set `self.LHandLerpAlpha` (`KismetMathLibrary.FClamp` (- (`self.LHandLerpAlpha`) (* (`self.Delta Seconds`) 2.0))))
    (`SceneComponent.K2_SetRelativeTransform` (`self.LHand`) (`KismetMathLibrary.TLerp` (`self.LHandLookTransform`) (`self.LHandRestTransform`) (`self.LHandLerpAlpha`)) false false)
    (if (<= (`self.LHandLerpAlpha`) 0.0)
      (`self.LHandStateChange` "NewEnumerator0")))
  (:`Completed`
    (switch `/Game/TrickPhotography/Programmers/Enums/ELHandState` (`self.LHandState`)
      (:`NewEnumerator0`
        _)
      (:`NewEnumerator3`
        _))
    (`self.LHandStateChange` "NewEnumerator1")))

(event `EnhancedInput|/Game/TrickPhotography/Programmers/Core/Inputs/IA_LookAtCamera`
  (params (ActionValue :type Boolean) (ElapsedSeconds :type "Float (double-precision)") (TriggeredSeconds :type "Float (double-precision)") (InputAction :type "InputAction Object Reference" :default "/Game/TrickPhotography/Programmers/Core/Inputs/IA_LookAtCamera.IA_LookAtCamera"))
  (:`Triggered`
    (switch `/Game/TrickPhotography/Programmers/Enums/ELHandState` (`self.LHandState`)
      (:`NewEnumerator2`
        (switch `/Game/TrickPhotography/Programmers/Enums/ERHandState` (`self.RHandState`)
          (:`NewEnumerator1`
            (`self.RHandStateChange` "NewEnumerator3"
              (:`ExecOut`
                _)))
          (:`NewEnumerator3`
            _))
        (set `self.RHandLerpAlpha` (`KismetMathLibrary.FClamp` (- (`self.RHandLerpAlpha`) (* (`self.Delta Seconds`) 2.0))))
        (`SceneComponent.K2_SetRelativeTransform` (`self.RHand`) (`KismetMathLibrary.TLerp` (`self.RHandLookTransform`) (`self.RHandRestTransform`) (`self.RHandLerpAlpha`)) false false)
        (if (<= (`self.RHandLerpAlpha`) 0.0)
          (`self.RHandStateChange` "NewEnumerator0"
            (:`ExecOut`
              (`self.SetCammyRotVis`)))))))
  (:`Completed`
    (switch `/Game/TrickPhotography/Programmers/Enums/ERHandState` (`self.RHandState`)
      (:`NewEnumerator0`
        _)
      (:`NewEnumerator3`
        _))
    (`self.RHandStateChange` "NewEnumerator1"
      (:`ExecOut`
        (`self.SetCammyRotVis`)))))

(event `EnhancedInput|/Game/TrickPhotography/Programmers/Core/Inputs/IA_SnapPhoto`
  (params (ActionValue :type Boolean) (ElapsedSeconds :type "Float (double-precision)") (TriggeredSeconds :type "Float (double-precision)") (InputAction :type "InputAction Object Reference" :default "/Game/TrickPhotography/Programmers/Core/Inputs/IA_SnapPhoto.IA_SnapPhoto"))
  (:`Started`
    (switch `/Game/TrickPhotography/Programmers/Enums/ERHandState` (`self.RHandState`)
      (:`NewEnumerator0`
        (`/Game/TrickPhotography/Programmers/Core/Camera/BP_FilterCamera.TakePhotoAsCammy` (`self.Camera`) (`self.CammyChar`) (`/Game/TrickPhotography/Programmers/Core/Player/MainPlayerController.SelectedFilter` (`self.PlayerController`)))
        (`KismetSystemLibrary.DelayUntilNextTick`)
        (`self.RHandStateChange` "NewEnumerator1"
          (:`ExecOut`
            (`self.SetCammyRotVis`)
            (bind _pickupgiven (`/Game/TrickPhotography/Programmers/Core/Player/BP_CammyCharacter.GiveAwayPhotos` (`self.CammyChar`)))
            (`self.AttachObjectToLHand` _pickupgiven)))))))

(event `EnhancedInput|/Game/TrickPhotography/Programmers/Core/Inputs/IA_DropPlacePhoto`
  (params (ActionValue :type Boolean) (ElapsedSeconds :type "Float (double-precision)") (TriggeredSeconds :type "Float (double-precision)") (InputAction :type "InputAction Object Reference" :default "/Game/TrickPhotography/Programmers/Core/Inputs/IA_DropPlacePhoto.IA_DropPlacePhoto"))
  (:`Started`
    (`self.DropObject`)))

(event `EnhancedInput|/Game/TrickPhotography/Programmers/Core/Inputs/IA_Interact`
  (params (ActionValue :type Boolean) (ElapsedSeconds :type "Float (double-precision)") (TriggeredSeconds :type "Float (double-precision)") (InputAction :type "InputAction Object Reference" :default "/Game/TrickPhotography/Programmers/Core/Inputs/IA_Interact.IA_Interact"))
  (:`Triggered`
    (`self.CheckInteractionInRange`))
  (:`Started`
    (`self.LineTraceInteractPickup`))
  (:`Canceled`
    (`self.EndInteract` :!label _label_5))
  (:`Completed`
    (goto _label_5)))

(event `EnhancedInput|/Game/TrickPhotography/Programmers/Core/Inputs/IA_PlaceCammy`
  (params (ActionValue :type Boolean) (ElapsedSeconds :type "Float (double-precision)") (TriggeredSeconds :type "Float (double-precision)") (InputAction :type "InputAction Object Reference" :default "/Game/TrickPhotography/Programmers/Core/Inputs/IA_PlaceCammy.IA_PlaceCammy"))
  (:`Started`
    (switch `/Game/TrickPhotography/Programmers/Enums/ERHandState` (`self.RHandState`)
      (:`NewEnumerator1`
        (switch `/Game/TrickPhotography/Programmers/Enums/ELHandState` (`self.LHandState`)
          (:`NewEnumerator1`
            _)
          (:`NewEnumerator2`
            _))
        (`/Game/TrickPhotography/Programmers/Core/Player/BP_CammyCharacter.Place` (`self.CammyChar`))
        (`self.RHandStateChange` "NewEnumerator2")))))

(event `TryHoldCammy`
  (switch `/Game/TrickPhotography/Programmers/Enums/ERHandState` (`self.RHandState`)
    (:`NewEnumerator2`
      (`/Game/TrickPhotography/Programmers/Core/Player/MainPlayerController.PossessMainCharacter` (`self.PlayerController`))
      (`/Game/TrickPhotography/Programmers/Core/Player/BP_CammyCharacter.Recall` (`self.CammyChar`) self)
      (`self.RHandStateChange` "NewEnumerator1"))))

(event `EnhancedInput|/Game/TrickPhotography/Programmers/Core/Inputs/Vault/IA_TurnDial`
  (params (ActionValue :type "Float (double-precision)") (ElapsedSeconds :type "Float (double-precision)") (TriggeredSeconds :type "Float (double-precision)") (InputAction :type "InputAction Object Reference" :default "/Game/TrickPhotography/Programmers/Core/Inputs/Vault/IA_TurnDial.IA_TurnDial"))
  (:`Triggered`
    (bind _asbp_vault (cast `/Game/TrickPhotography/Programmers/Puzzles/BP_Vault` (`self.LookingAtInteract`)))
    (`/Game/TrickPhotography/Programmers/Puzzles/BP_Vault.RotateWheel` _asbp_vault 0 (== ActionValue 1.0))))

(fn `AttachObjectToLHand`
  (params (ObjectToAttach :type "PickupableInterface Interface"))
  (if (`KismetSystemLibrary.IsValidInterface` ObjectToAttach)
    (bind _returnvalue (`PickupableInterface.CanBePickedUp` ObjectToAttach false))
    (if _returnvalue
      (`PickupableInterface.OnPickup` ObjectToAttach false)
      ; Double check that it's still valid and pickupable - the item might destroy itself once it's notified of being picked up
      (`/Engine/EditorBlueprintResources/StandardMacros.IsValid` (`KismetSystemLibrary.Conv_InterfaceToObject` ObjectToAttach)
        (:`Is Valid`
          (bind _returnvalue_2 (`PickupableInterface.CanBePickedUp` ObjectToAttach false))
          (if _returnvalue_2
            (bind _aspickup (cast `Pickup` ObjectToAttach))
            (switch `/Game/TrickPhotography/Programmers/Enums/ELHandState` (`self.LHandState`)
              (:`NewEnumerator0`
                (`self.SwapObject` _aspickup (`self.HeldObject`) :!label _label))
              (:`NewEnumerator1`
                (goto _label))
              (:`NewEnumerator2`
                _)
              (:`NewEnumerator3`
                (goto _label)))
            (set `self.CurrentPickup` ObjectToAttach)
            (bind _output_get (set `self.HeldObject` _aspickup))
            (bind _returnvalue_3 (`self.K2_AttachToComponent` _output_get (`self.LHand`) "Hand" "SnapToTarget" "SnapToTarget" "KeepRelative" false))
            (if _returnvalue_3
              (`self.LHandStateChange` "NewEnumerator1"
                (:`ExecOut`
                  (`KismetSystemLibrary.PrintString` "Attached!")))
              (else
                (`KismetSystemLibrary.PrintString` "failed")))))))))

(fn `CheckInteractionInRange`
  (bind _asactor (cast `Actor` (`self.CurrentInteract`)))
  (if (> (`KismetMathLibrary.Vector_Distance` (`self.K2_GetActorLocation` _asactor) (`SceneComponent.K2_GetComponentLocation` (`self.FirstPersonCamera`))) (`self.InteractRange`))
    (`self.EndInteract`)))

(fn `DetachHeldObject`
  (`/Engine/EditorBlueprintResources/StandardMacros.IsValid` (`self.HeldObject`)
    (:`Is Valid`
      (`self.K2_DetachFromActor` (`self.HeldObject`) "KeepWorld" "KeepWorld" "KeepRelative")
      (set `self.HeldObject` null)
      (set `self.CurrentPickup` null)
      (`self.LHandStateChange` "NewEnumerator2"))
    (:`Is Not Valid`
      (`KismetSystemLibrary.PrintString` "No object to detach"))))

(fn `DropObject`
  (bind _heldobject (`self.HeldObject`))
  (switch `/Game/TrickPhotography/Programmers/Enums/ERHandState` (`self.RHandState`)
    (:`NewEnumerator1`
      _)
    (:`NewEnumerator2`
      _))
  (switch `/Game/TrickPhotography/Programmers/Enums/ELHandState` (`self.LHandState`)
    (:`NewEnumerator0`
      _)
    (:`NewEnumerator1`
      _)
    (:`NewEnumerator3`
      _))
  (`/Engine/EditorBlueprintResources/StandardMacros.IsValid` _heldobject
    (:`Is Valid`
      (`self.K2_DetachFromActor` _heldobject "KeepWorld" "KeepWorld" "KeepWorld")
      (`PickupableInterface.OnDrop` (`self.CurrentPickup`) false)
      (bind _asprimitive_component (cast `PrimitiveComponent` (`Actor.RootComponent` (`self.HeldObject`)))
        (:`then`
          (`PrimitiveComponent.AddForce` _asprimitive_component (* (`self.GetActorForwardVector`) 10000.0) "None" false))
        (:`CastFailed`
          (`KismetSystemLibrary.PrintString` "Hello")))
      (set `self.HeldObject` null)
      (set `self.CurrentPickup` null)
      (`self.LHandStateChange` "NewEnumerator2"))))

(fn `EndInteract`
  (bind _currentinteract (`self.CurrentInteract`))
  (if (`KismetSystemLibrary.IsValidInterface` _currentinteract)
    (`/Game/TrickPhotography/Programmers/Core/Interfaces/BPI_Interactable.InteractEnd` _currentinteract false)
    (set `self.CurrentInteract` null)))

(fn `LineTraceInteractPickup`
  (bind _heldobject (`self.HeldObject`))
  (bind _currentpickup (`self.CurrentPickup`))
  (bind _firstpersoncamera (`self.FirstPersonCamera`))
  (bind _returnvalue (`SceneComponent.K2_GetComponentLocation` _firstpersoncamera))
  (switch `/Game/TrickPhotography/Programmers/Enums/ELHandState` (`self.LHandState`)
    (:`NewEnumerator1`
      _)
    (:`NewEnumerator2`
      _))
  (switch `/Game/TrickPhotography/Programmers/Enums/ERHandState` (`self.RHandState`)
    (:`NewEnumerator1`
      _)
    (:`NewEnumerator2`
      _))
  (bind (_outhit _returnvalue_2) (`KismetSystemLibrary.LineTraceSingle` _returnvalue (+ _returnvalue (* (`KismetMathLibrary.GetForwardVector` (`SceneComponent.K2_GetComponentRotation` _firstpersoncamera)) (`self.InteractRange`))) "TraceTypeQuery1" true))
  (if _returnvalue_2
    (bind _asbpi_interactable (cast `/Game/TrickPhotography/Programmers/Core/Interfaces/BPI_Interactable` (`.HitActor` (`GameplayStatics.BreakHitResult` _outhit)))
      (:`then`
        (bind _output_get (set `self.CurrentInteract` _asbpi_interactable))
        (`/Game/TrickPhotography/Programmers/Core/Interfaces/BPI_Interactable.InteractStart` _output_get (`self.CurrentPickup`) false))
      (:`CastFailed`
        (bind _aspickupable_interface (cast `PickupableInterface` (`.HitActor` (`GameplayStatics.BreakHitResult` _outhit)))
          (:`then`
            (bind _aspickup (cast `Pickup` _aspickupable_interface))
            (if (== (`self.CammyChar`) (`self.GetAttachParentActor` _aspickup))
              (`self.DropObject`)
              (bind _pickupgiven (`/Game/TrickPhotography/Programmers/Core/Player/BP_CammyCharacter.GiveAwayPhotos` (`self.CammyChar`)))
              (`self.AttachObjectToLHand` _pickupgiven)
              (else
                (`self.AttachObjectToLHand` _aspickupable_interface))))
          (:`CastFailed`
            (bind _asbp_cammy_character (cast `/Game/TrickPhotography/Programmers/Core/Player/BP_CammyCharacter` (`.HitActor` (`GameplayStatics.BreakHitResult` _outhit)))
              (:`then`
                (`self.TryHoldCammy`)
                (bind _pickupgiven_2 (`/Game/TrickPhotography/Programmers/Core/Player/BP_CammyCharacter.GiveAwayPhotos` _asbp_cammy_character))
                (`self.AttachObjectToLHand` _pickupgiven_2))
              (:`CastFailed`
                (cast `StaticMeshActor` (`.HitActor` (`GameplayStatics.BreakHitResult` _outhit))
                  (:`then`
                    (cast `/Game/TrickPhotography/Programmers/Core/Camera/BP_Photograph` _heldobject
                      (:`then`
                        (`self.PlaceObject` _heldobject (`KismetMathLibrary.MakeTransform` (+ (`.Location` (`GameplayStatics.BreakHitResult` _outhit)) (* (`.Normal` (`GameplayStatics.BreakHitResult` _outhit)) (`KismetMathLibrary.RandomFloatInRange` 0.0 0.1))) (`KismetMathLibrary.ComposeRotators` (`KismetMathLibrary.MakeRotator` 0.0 0.0 (`KismetMathLibrary.RandomFloatInRange` 170.0 190.0)) (`KismetMathLibrary.MakeRotFromZ` (`.Normal` (`GameplayStatics.BreakHitResult` _outhit)))))))
                      (:`CastFailed`
                        ; Activate held item if applicable
                        (`/Engine/EditorBlueprintResources/StandardMacros.IsValid` (`KismetSystemLibrary.Conv_InterfaceToObject` _currentpickup) :!label _label
                          (:`Is Valid`
                            (`PickupableInterface.Activate` _currentpickup (`SceneComponent.K2_GetComponentToWorld` (`self.FirstPersonCamera`)) false))))))
                  (:`CastFailed`
                    (goto _label)))))))))
    (else
      (goto _label))))

(fn `PlaceObject`
  (params (PickupToPlace :type "Pickup Object Reference") (PositionToPlace :type "Transform Structure"))
  (locals (TempToPick :type "Pickup Object Reference") (TempToPlace :type "Pickup Object Reference"))
  (bind _temptoplace (`local.TempToPlace`))
  (set `local.TempToPlace` PickupToPlace)
  (switch `/Game/TrickPhotography/Programmers/Enums/ERHandState` (`self.RHandState`)
    (:`NewEnumerator1`
      _)
    (:`NewEnumerator2`
      _))
  (switch `/Game/TrickPhotography/Programmers/Enums/ELHandState` (`self.LHandState`)
    (:`NewEnumerator0`
      _)
    (:`NewEnumerator1`
      _)
    (:`NewEnumerator3`
      _))
  (`/Engine/EditorBlueprintResources/StandardMacros.IsValid` _temptoplace
    (:`Is Valid`
      (`self.K2_SetActorLocationAndRotation` _temptoplace PositionToPlace_Location PositionToPlace_Rotation false true)
      (`self.K2_DetachFromActor` _temptoplace "KeepWorld" "KeepWorld" "KeepWorld")
      (`PickupableInterface.OnDrop` (`self.CurrentPickup`) false)
      (bind _asbp_photograph (cast `/Game/TrickPhotography/Programmers/Core/Camera/BP_Photograph` _temptoplace)
        (:`then`
          (`/Game/TrickPhotography/Programmers/Core/Camera/BP_Photograph.SetAttachedToWall` _asbp_photograph true))
        (:`CastFailed`
          _))
      (set `self.HeldObject` null)
      (set `self.CurrentPickup` null)
      (`self.LHandStateChange` "NewEnumerator2"))))

(fn `SetCammyRotVis`
  (switch `/Game/TrickPhotography/Programmers/Enums/ERHandState` (`self.RHandState`)
    (:`NewEnumerator0`
      (`self.K2_SetActorRelativeRotation` (`self.CammyChar`) (`KismetMathLibrary.MakeRotator` 90.0 180.0 -90.0) false false)
      (`self.SetActorHiddenInGame` (`self.CammyChar`) true))
    (:`NewEnumerator1`
      (`self.K2_SetActorRelativeRotation` (`self.CammyChar`) (struct :`Yaw` -90.0 :`Roll` 90.0) false false :!label _label)
      (`self.SetActorHiddenInGame` (`self.CammyChar`) false))
    (:`NewEnumerator3`
      (goto _label))))

(fn `SwapObject`
  (params (PickupToPick :type "Pickup Object Reference") (PickupToPlace :type "Pickup Object Reference"))
  (locals (TempToPick :type "Pickup Object Reference") (TempToPlace :type "Pickup Object Reference"))
  (bind _temptoplace (`local.TempToPlace`))
  (bind _temptopick (`local.TempToPick`))
  (set `local.TempToPick` PickupToPick)
  (set `local.TempToPlace` PickupToPlace)
  (switch `/Game/TrickPhotography/Programmers/Enums/ERHandState` (`self.RHandState`)
    (:`NewEnumerator1`
      _)
    (:`NewEnumerator2`
      _))
  (switch `/Game/TrickPhotography/Programmers/Enums/ELHandState` (`self.LHandState`)
    (:`NewEnumerator0`
      _)
    (:`NewEnumerator1`
      _)
    (:`NewEnumerator3`
      _))
  (`/Engine/EditorBlueprintResources/StandardMacros.IsValid` _temptoplace
    (:`Is Valid`
      (`self.K2_SetActorLocationAndRotation` _temptoplace (`self.K2_GetActorLocation` _temptopick) (`self.K2_GetActorRotation` _temptopick) false true)
      (`self.K2_DetachFromActor` (`local.TempToPlace`) "KeepWorld" "KeepWorld" "KeepWorld")
      (`PickupableInterface.OnDrop` (`self.CurrentPickup`) false)
      (bind _asbp_photograph (cast `/Game/TrickPhotography/Programmers/Core/Camera/BP_Photograph` (`local.TempToPlace`))
        (:`then`
          (bind _asbp_photograph_2 (cast `/Game/TrickPhotography/Programmers/Core/Camera/BP_Photograph` (`local.TempToPick`))
            (:`then`
              (`/Game/TrickPhotography/Programmers/Core/Camera/BP_Photograph.SetAttachedToWall` _asbp_photograph (`/Game/TrickPhotography/Programmers/Core/Camera/BP_Photograph.bIsAttachedToWall` _asbp_photograph_2)))
            (:`CastFailed`
              _)))
        (:`CastFailed`
          _))
      (set `self.HeldObject` null)
      (set `self.CurrentPickup` null)
      (`self.LHandStateChange` "NewEnumerator2"))))

(fn `UserConstructionScript`)