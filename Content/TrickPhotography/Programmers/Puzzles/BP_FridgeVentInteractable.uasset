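; BP_FridgeVentInteractable is a puzzle interactable for a fridge vent that only responds when Cammy starts the interaction.
; On interaction it finds the BP_CammyCharacter, teleports it five units downward without sweeping, then activates the linked FridgeToActivate.
; Both hover functions always return false, and non-Cammy interactions do nothing.
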(event `/Game/TrickPhotography/Programmers/Core/Interfaces/BPI_Interactable.InteractStart`
  (params (HeldItem :type "PickupableInterface Interface") (bIsCammy :type Boolean) (HitComponent :type "PrimitiveComponent Object Reference"))
  (if bIsCammy
    (bind _returnvalue (`GameplayStatics.GetActorOfClass` "/Game/TrickPhotography/Programmers/Core/Player/BP_CammyCharacter.BP_CammyCharacter_C"))
    (`self.K2_SetActorLocation` _returnvalue (+ (`self.K2_GetActorLocation` _returnvalue) (0.0 0.0 -5.0)) false true)
    (`/Game/TrickPhotography/Programmers/Core/Interfaces/BPI_Activatable.Activate` (`self.FridgeToActivate`))))

(fn `HoverOngoing`
  (params (HeldItem :type "PickupableInterface Interface") (HitComponent :type "PrimitiveComponent Object Reference"))
  (returns (bIsInteractable :type Boolean))
  (return false))

(fn `HoverStart`
  (params (HeldItem :type "PickupableInterface Interface") (HitComponent :type "PrimitiveComponent Object Reference"))
  (returns (bIsInteractable :type Boolean))
  (return false))

(fn `UserConstructionScript`)