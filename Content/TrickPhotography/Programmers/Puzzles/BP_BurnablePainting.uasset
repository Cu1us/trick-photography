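; BP_BurnablePainting is a puzzle painting that burns away from a given point and then destroys itself.
; BeginPlay creates a dynamic M_BurnFromPoint material on the Canvas and applies the painting's texture.
; Burn runs once, passing the start point to the material, showing a decal there and enabling tick.
; Tick grows the material's burn distance at BurnRate until it passes a threshold and the actor is destroyed.
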(event `self.ReceiveBeginPlay`
  (`/Engine/EditorBlueprintResources/StandardMacros.IsValid` (`self.MaterialInstance`)
    (:`Is Valid`)
    (:`Is Not Valid`
      (bind _returnvalue (`PrimitiveComponent.CreateDynamicMaterialInstance` (`self.Canvas`) 0 "/Game/TrickPhotography/Art/Enviroment/Enviroment_Shaders/M_BurnFromPoint.M_BurnFromPoint" "None"))
      (`MaterialInstanceDynamic.SetTextureParameterValue` _returnvalue "MainTexture" (`self.Texture`))
      (set `self.MaterialInstance` _returnvalue))))

(event `Burn`
  (params (StartPoint :type "Vector Structure"))
  (bind _decal (`self.Decal`))
  (if (not (`self.bBurning`))
    (set `self.bBurning` true)
    (`MaterialInstanceDynamic.SetVectorParameterValue` (`self.MaterialInstance`) "BurnSource" (`KismetMathLibrary.Conv_VectorToLinearColor` StartPoint))
    (`self.SetActorTickEnabled` true)
    (set `self.BurnProgress` 0.0)
    (`SceneComponent.K2_SetWorldLocation` _decal StartPoint false false)
    (`SceneComponent.SetVisibility` _decal true false)))

(event `self.ReceiveTick`
  (params (DeltaSeconds :type "Float (single-precision)"))
  (if (`self.bBurning`)
    (bind _output_get (set `self.BurnProgress` (+ (`self.BurnProgress`) (* DeltaSeconds (`self.BurnRate`)))))
    (`MaterialInstanceDynamic.SetScalarParameterValue` (`self.MaterialInstance`) "BurnDistance" _output_get)
    (if (> _output_get (`self.BurnDeleteThreshold`))
      (`self.K2_DestroyActor`))))

(fn `UserConstructionScript`)