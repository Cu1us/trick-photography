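; BP_LightSwitch is an interactable puzzle switch that depends on a breaker box for power.
; On interact, it toggles between activated and deactivated if the breaker box is activated, and otherwise prints a "no power" message.
; At BeginPlay it binds to the breaker box's deactivation event, so it switches itself off when power is cut.
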(event `self.ReceiveBeginPlay`
  ; Deactivate is breaker is suddenly turned off
  (add `self.OnDeactivated` (`self.BreakerBox`) (delegate `BreakerBoxDeactivated`)))

(event `BreakerBoxDeactivated`
  ; Deactivate is breaker is suddenly turned off
  (if (`self.bIsActivated`)
    (`self.Deactivate`)))

(event `/Game/TrickPhotography/Programmers/Core/Interfaces/BPI_Interactable.InteractStart`
  (params (HeldItem :type "PickupableInterface Interface"))
  ; Only activates if breaker box is activated
  (if (`/Game/TrickPhotography/Programmers/Core/BaseClasses/BP_ActivatorBase.bIsActivated` (`self.BreakerBox`))
    ; Toggles activation status
    (if (`self.bIsActivated`)
      (`self.Deactivate`)
      (else
        (`self.Activate`)))
    (else
      (`KismetSystemLibrary.PrintString` "no power"))))

(fn `UserConstructionScript`
  (`parent.UserConstructionScript`))