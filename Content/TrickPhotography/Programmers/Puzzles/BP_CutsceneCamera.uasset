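; Puzzle cutscene camera pawn that starts animating on possession and fires OnAnimationFinished after an end delay.
; Tick compares advanced time against zero rather than track duration, so it normally jumps to the duration and stops on the first tick.
; SetAnimationTime teleports the camera to the Track spline transform at that time, rotated toward FocusPoint when valid.
; Tick updates only the time variable, without calling SetAnimationTime.
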(event `self.ReceivePossessed`
  (params (NewController :type "Controller Object Reference"))
  (set `self.bIsAnimating` true)
  (set `self.AnimationTime` 0.0))

(event `self.ReceiveUnpossessed`
  (params (OldController :type "Controller Object Reference"))
  (set `self.bIsAnimating` false))

(event `self.ReceiveTick`
  (params (DeltaSeconds :type "Float (single-precision)"))
  (bind _returnvalue (+ (`self.AnimationTime`) DeltaSeconds))
  (bind _returnvalue_2 (>= _returnvalue 0.0))
  (if (`self.bIsAnimating`)
    (set `self.AnimationTime` (`KismetMathLibrary.SelectFloat` (`SplineComponent.Duration` (`self.Track`)) _returnvalue _returnvalue_2))
    (if _returnvalue_2
      (set `self.bIsAnimating` false)
      (`KismetSystemLibrary.Delay` (`self.WaitTimeAtEnd`))
      (`self.OnAnimationFinished`))))

(fn `GetCameraLocationByTime`
  (params (Time :type "Float (double-precision)"))
  (returns (ReturnValue :type "Transform Structure"))
  (bind _focuspoint (`self.FocusPoint`))
  (bind _returnvalue (`SplineComponent.GetTransformAtTime` (`self.Track`) Time "World" false false))
  (bind _returnvalue_location (`KismetMathLibrary.BreakTransform` (`self.GetTransform` _focuspoint)))
  (bind _location (.location _returnvalue))
  (`/Engine/EditorBlueprintResources/StandardMacros.IsValid` _focuspoint
    (:`Is Valid`
      (return (`KismetMathLibrary.MakeTransform` _location (`KismetMathLibrary.FindLookAtRotation` _location _returnvalue_location) (.scale _returnvalue))))
    (:`Is Not Valid`
      (return _returnvalue))))

(fn `SetAnimationTime`
  (params (NewTime :type "Float (double-precision)"))
  (bind _output_get (set `self.AnimationTime` NewTime))
  (bind _returnvalue (`self.GetCameraLocationByTime` _output_get))
  (`SceneComponent.K2_SetWorldTransform` (`self.Camera`) _returnvalue false true))

(fn `UserConstructionScript`)