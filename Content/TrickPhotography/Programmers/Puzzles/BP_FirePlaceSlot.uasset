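; BP_FirePlaceSlot is an interactable puzzle fireplace slot that receives a log and can then be lit.
; Overlapping BP_LogPickup actors are notified with the slot, and SetLogInFireplace reveals the hidden Log mesh while disabling the Box collision.
; Interacting activates any held item from the first-person camera transform; empty-handed, it lights the PointLight if the Log was hit.
; Hover sets the player's prompt based on the hit component and held item.
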(event `self.ReceiveBeginPlay`
  (`parent.ReceiveBeginPlay`)
  (`PrimitiveComponent.SetCollisionEnabled` (`self.Log`) "NoCollision")
  (`SceneComponent.SetVisibility` (`self.Log`) false false)
  (bind _asmain_player_controller (cast `/Game/TrickPhotography/Programmers/Core/Player/MainPlayerController` (`GameplayStatics.GetPlayerController` 0)))
  (set `self.MainPlayerController` _asmain_player_controller))

(event `SetLogInFireplace`
  (`SceneComponent.SetVisibility` (`self.Log`) true false)
  (`PrimitiveComponent.SetCollisionEnabled` (`self.Log`) "QueryAndPhysics")
  (`PrimitiveComponent.SetCollisionEnabled` (`self.Box`) "NoCollision"))

(event `/Game/TrickPhotography/Programmers/Core/Interfaces/BPI_Interactable.InteractStart`
  (params (HeldItem :type "PickupableInterface Interface") (bIsCammy :type Boolean) (HitComponent :type "PrimitiveComponent Object Reference"))
  (if (`KismetSystemLibrary.IsValidInterface` HeldItem)
    (`PickupableInterface.Activate` HeldItem (`SceneComponent.K2_GetComponentToWorld` (`/Game/TrickPhotography/Programmers/Core/Player/BP_MainCharacter.FirstPersonCamera` (`/Game/TrickPhotography/Programmers/Core/Player/MainPlayerController.MainChar` (`self.MainPlayerController`)))) bIsCammy)
    (else
      (`SceneComponent.SetVisibility` (`self.PointLight`) (== HitComponent (`self.Log`)) false)
      (`PrimitiveComponent.SetCollisionEnabled` (`self.Log`) "NoCollision"))))

(event `self.ReceiveActorBeginOverlap`
  (params (OtherActor :type "Actor Object Reference"))
  (bind _asbp_log_pickup (cast `/Game/TrickPhotography/Programmers/Pickups/BP_LogPickup` OtherActor))
  (`/Game/TrickPhotography/Programmers/Pickups/BP_LogPickup.LogCollidedWithFireplaceSlot` _asbp_log_pickup self))

(fn `HoverOngoing`
  (params (HeldItem :type "PickupableInterface Interface") (HitComponent :type "PrimitiveComponent Object Reference"))
  (returns (bIsInteractable :type Boolean))
  (cast `/Game/TrickPhotography/Programmers/Pickups/BP_LogPickup` HeldItem
    (:`then`
      (return true))
    (:`CastFailed`
      (return true))))

(fn `HoverStart`
  (params (HeldItem :type "PickupableInterface Interface") (HitComponent :type "PrimitiveComponent Object Reference"))
  (returns (bIsInteractable :type Boolean))
  (bind _asmain_player_controller (cast `/Game/TrickPhotography/Programmers/Core/Player/MainPlayerController` (`GameplayStatics.GetPlayerController` 0)))
  (if (== HitComponent (`self.Log`))
    (bind _mainchar (`/Game/TrickPhotography/Programmers/Core/Player/MainPlayerController.MainChar` _asmain_player_controller))
    (set `/Game/TrickPhotography/Programmers/Core/Player/BP_MainCharacter.InteractOverrideText` "Light Fire \n" _mainchar)
    (else
      (cast `/Game/TrickPhotography/Programmers/Pickups/BP_LogPickup` HeldItem
        (:`then`
          (set `/Game/TrickPhotography/Programmers/Core/Player/BP_MainCharacter.InteractOverrideText` "Place Log \n" _mainchar))
        (:`CastFailed`
          (set `/Game/TrickPhotography/Programmers/Core/Player/BP_MainCharacter.InteractOverrideText` "Need wood" _mainchar)))))
  (return true))

(fn `UserConstructionScript`)