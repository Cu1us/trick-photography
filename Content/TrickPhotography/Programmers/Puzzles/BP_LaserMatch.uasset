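; BP_LaserMatch is a puzzle match that lights once when its Light event is called.
; Light sets a Lit flag, shows the Flame and PointLight components, then runs a short delay with nothing after it.
; A disconnected chain would swap the match for a burned version and play FireTimeline, and the LightBuildup event is empty.
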(event `Light`
  (if (not (`self.bLit`))
    (set `self.bLit` true)
    (`SceneComponent.SetVisibility` (`self.Flame`) true false)
    (`SceneComponent.SetVisibility` (`self.PointLight`) true false)
    (`KismetSystemLibrary.Delay` 0.2)))

(event `LightBuildup`)

(fn `UserConstructionScript`)