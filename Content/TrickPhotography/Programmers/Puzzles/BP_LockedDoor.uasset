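; BP_LockedDoor is an interactable puzzle door that swings open when a matching key pickup is used on its keyhole.
; InteractStart ignores Cammy interactions, requires a hit on KeyHole, and compares the held Pickup's ID to PickupIDReq.
; A match makes the main character drop the item and plays a Timeline that offsets actor yaw from the rotation cached at BeginPlay.
; Both hover functions return false.
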(event `self.ReceiveBeginPlay`
  (bind (_returnvalue_roll _returnvalue_pitch _returnvalue_yaw) (`KismetMathLibrary.BreakRotator` (`self.K2_GetActorRotation`)))
  (`parent.ReceiveBeginPlay`)
  (set `self.InitialRot` _returnvalue_yaw))

(event `/Game/TrickPhotography/Programmers/Core/Interfaces/BPI_Interactable.InteractStart`
  (params (HeldItem :type "PickupableInterface Interface") (bIsCammy :type Boolean) (HitComponent :type "PrimitiveComponent Object Reference"))
  (bind (_returnvalue_roll _returnvalue_pitch) (`KismetMathLibrary.BreakRotator` (`self.K2_GetActorRotation`)))
  (if bIsCammy
    _
    (elif (== HitComponent (`self.KeyHole`))
      (bind _aspickup (cast `Pickup` HeldItem))
      (if (`KismetStringLibrary.EqualEqual_StrStr` (`self.PickupIDReq`) (`Pickup.PickupID` _aspickup))
        (bind _asmain_player_controller (cast `/Game/TrickPhotography/Programmers/Core/Player/MainPlayerController` (`GameplayStatics.GetPlayerController` 0)))
        (`/Game/TrickPhotography/Programmers/Core/Player/BP_MainCharacter.DropObject` (`/Game/TrickPhotography/Programmers/Core/Player/MainPlayerController.MainChar` _asmain_player_controller) true)
        (bind (_direction _z) (`Timeline|Timeline`)
          (:`Update`
            (`self.K2_SetActorRotation` (`KismetMathLibrary.MakeRotator` _returnvalue_roll _returnvalue_pitch (+ _z (`self.InitialRot`))))))))))

(fn `HoverOngoing`
  (params (HeldItem :type "PickupableInterface Interface") (HitComponent :type "PrimitiveComponent Object Reference"))
  (returns (bIsInteractable :type Boolean))
  (return false))

(fn `HoverStart`
  (params (HeldItem :type "PickupableInterface Interface") (HitComponent :type "PrimitiveComponent Object Reference"))
  (returns (bIsInteractable :type Boolean))
  (return false))

(fn `UserConstructionScript`)