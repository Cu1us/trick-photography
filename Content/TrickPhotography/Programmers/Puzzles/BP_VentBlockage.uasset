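; Puzzle interactable for a vent blockage that only Cammy can highlight and clear, teleporting that character to a linked EndPoint.
; Interacting disables the collider, destroys the blocking meshes, switches filterable decals from hot to cold color and triggers the EndPoint's own interaction.
; With a valid VentDoor, it also spawns configured objects at TargetPoint and uses timelines to swing the door open, then back after a delay.
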(event `self.ReceiveBeginPlay`
  (bind _asmain_player_controller (cast `/Game/TrickPhotography/Programmers/Core/Player/MainPlayerController` (`GameplayStatics.GetPlayerController` 0)))
  (set `self.Teleporting Actor` (`/Game/TrickPhotography/Programmers/Core/Player/MainPlayerController.CammyChar` _asmain_player_controller))
  (for _array_element (`self.DecalsToSetColorOn`)
    (bind _asfilterable_decal_actor (cast `FilterableDecalActor` _array_element))
    (`DecalComponent.SetDecalColor` (`DecalActor.Decal` _asfilterable_decal_actor) (`self.HotColor`))))

(event `/Game/TrickPhotography/Programmers/Core/Interfaces/BPI_Interactable.InteractStart`
  (params (HeldItem :type "PickupableInterface Interface") (bIsCammy :type Boolean) (HitComponent :type "PrimitiveComponent Object Reference"))
  (bind _endpoint (`self.EndPoint`))
  (bind (_ventrot_roll _ventrot_pitch _ventrot_yaw) (`KismetMathLibrary.BreakRotator` (`self.VentRot`)))
  (bind (_ventrot_roll_2 _ventrot_pitch_2 _ventrot_yaw_2) (`KismetMathLibrary.BreakRotator` (`self.VentRot`)))
  (bind _ventdoor (`self.VentDoor`))
  (if bIsCammy
    (`/Engine/EditorBlueprintResources/StandardMacros.IsValid` (`self.EndPoint`)
      (:`Is Valid`
        (`self.K2_SetActorLocation` (`self.Teleporting Actor`) (`self.K2_GetActorLocation` (`self.EndPoint`)) false true))
      (:`Is Not Valid`
        _))
    (`PrimitiveComponent.SetCollisionEnabled` (`self.Collider`) "NoCollision")
    (`/Engine/EditorBlueprintResources/StandardMacros.IsValid` (`self.VentDoor`)
      (:`Is Valid`
        (for _array_element (`self.ObjectsToSpawnOnOpen`)
          (`|SpawnActorFromClass` _array_element (`KismetMathLibrary.MakeTransform` (`self.K2_GetActorLocation` (`self.TargetPoint`))) "AlwaysSpawn" "MultiplyWithRoot" null null)))
      (:`Is Not Valid`
        _))
    (for _array_element_2 (`SceneComponent.GetChildrenComponents` (`self.BlockingObjectsReplaceMeshes`) true)
      (`ActorComponent.K2_DestroyComponent` _array_element_2))
    (`ActorComponent.K2_DestroyComponent` (`self.BlockingObjectsReplaceMeshes`))
    (for _array_element_3 (`self.DecalsToSetColorOn`)
      (bind _asfilterable_decal_actor (cast `FilterableDecalActor` _array_element_3))
      (`DecalComponent.SetDecalColor` (`DecalActor.Decal` _asfilterable_decal_actor) (`self.ColdColor`)))
    (`/Engine/EditorBlueprintResources/StandardMacros.IsValid` _endpoint
      (:`Is Valid`
        (`/Game/TrickPhotography/Programmers/Core/Interfaces/BPI_Interactable.InteractStart` _endpoint null true null))
      (:`Is Not Valid`
        _))
    (`/Engine/EditorBlueprintResources/StandardMacros.IsValid` _ventdoor
      (:`Is Valid`
        (set `self.VentRot` (`self.K2_GetActorRotation` _ventdoor))
        (bind (_direction _rot) (`Timeline|Timeline`)
          (:`Update`
            (`self.K2_SetActorRotation` (`self.VentDoor`) (`KismetMathLibrary.MakeRotator` (+ _ventrot_roll_2 _rot) _ventrot_pitch_2 _ventrot_yaw_2) false))
          (:`Finished`
            (`KismetSystemLibrary.Delay` 2.0)
            (set `self.VentRot` (`self.K2_GetActorRotation` (`self.VentDoor`)))
            (`KismetSystemLibrary.PrintString` "Close")
            (bind (_direction_2 _rot_2) (`Timeline|Timeline_0`)
              (:`Update`
                (`self.K2_SetActorRotation` (`self.VentDoor`) (`KismetMathLibrary.MakeRotator` (- _ventrot_roll _rot_2) _ventrot_pitch _ventrot_yaw) false)))))))))

(event `/Game/TrickPhotography/Programmers/Core/Interfaces/BPI_Interactable.HoverEnd`
  (params (HeldItem :type "PickupableInterface Interface") (bIsCammy :type Boolean))
  (if bIsCammy
    (`self.SetPPMHighlight` "None")))

(fn `HoverOngoing`
  (params (HeldItem :type "PickupableInterface Interface") (HitComponent :type "PrimitiveComponent Object Reference"))
  (returns (bIsInteractable :type Boolean))
  (return false))

(fn `HoverStart`
  (params (HeldItem :type "PickupableInterface Interface") (HitComponent :type "PrimitiveComponent Object Reference") (bIsCammy :type Boolean))
  (returns (bIsInteractable :type Boolean))
  (if bIsCammy
    (`self.SetPPMHighlight` "HighlightPickup")
    (return false)))

(fn `UserConstructionScript`)