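; BP_PortalPolariodCamera is a puzzle camera that captures the scene into a render target for a photograph material.
; On BeginPlay, if no render target is set, it creates one at Resolution, plus a dynamic M_Photograph_Photo material showing it if PhotoMaterial is also unset.
; It then assigns the target to SceneCapture and captures once through Render, which can be called again to refresh the image.
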(event `self.ReceiveBeginPlay`
  (bind _resolution (`self.Resolution`))
  (`/Engine/EditorBlueprintResources/StandardMacros.IsValid` (`self.RenderTarget`)
    (:`Is Valid`
      _)
    (:`Is Not Valid`
      (bind _returnvalue (`KismetRenderingLibrary.CreateRenderTarget2D` _resolution _resolution "RTF_RGBA16f" (struct :`R` 1.0 :`B` 0.638639 :`A` 1.0)))
      (bind _output_get (set `self.RenderTarget` _returnvalue))
      (`/Engine/EditorBlueprintResources/StandardMacros.IsValid` (`self.PhotoMaterial`)
        (:`Is Valid`
          _)
        (:`Is Not Valid`
          (bind _returnvalue_2 (`KismetMaterialLibrary.CreateDynamicMaterialInstance` "/Game/TrickPhotography/Art/Enviroment/Materials_MeshSpecific/Photograph/M_Photograph_Photo.M_Photograph_Photo" "None" "Transient"))
          (`MaterialInstanceDynamic.SetTextureParameterValue` _returnvalue_2 "Image" _output_get)
          (`MaterialInstanceDynamic.SetScalarParameterValue` _returnvalue_2 "Opacity" 1.0)
          (set `self.PhotoMaterial` _returnvalue_2)))))
  (set `SceneCaptureComponent2D.TextureTarget` (`self.RenderTarget`) (`self.SceneCapture`))
  (`self.Render`))

(fn `Render`
  (`SceneCaptureComponent2D.CaptureScene` (`self.SceneCapture`)))

(fn `UserConstructionScript`)