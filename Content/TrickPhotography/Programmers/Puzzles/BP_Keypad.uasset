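; Interactable keypad puzzle that takes a PIN from non-Cammy interactions and fires its activation when the code matches.
; The hit component selects confirm, cancel or a digit parsed from its name, while ABP_Keypad animates the held key.
; Digits update the text display and auto-confirm once the code length is reached.
; A wrong code locks input while a delayable loop flashes the fail material, then clears the entry.
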(event `/Game/TrickPhotography/Programmers/Core/Interfaces/BPI_Interactable.InteractEnd`
  (params (bIsCammy :type Boolean) (HitComponent :type "PrimitiveComponent Object Reference"))
  (if (and (not bIsCammy) (!= (`self.HeldButton`) -1))
    (`self.SetButton` (`self.HeldButton`))))

(event `/Game/TrickPhotography/Programmers/Core/Interfaces/BPI_Interactable.InteractStart`
  (params (HeldItem :type "PickupableInterface Interface") (bIsCammy :type Boolean) (HitComponent :type "PrimitiveComponent Object Reference"))
  (bind _returnvalue (`KismetSystemLibrary.GetObjectName` HitComponent))
  (bind _returnvalue_2 (`KismetStringLibrary.Conv_StringToInt` _returnvalue))
  (if bIsCammy
    _
    (elif (`self.bIgnoreInputs`)
      _
      (elif (== HitComponent (`self.Confirm`))
        (`self.ConfirmCode`)
        (`self.SetButton` 11 true)
        (elif (== HitComponent (`self.Cancel`))
          (`self.ClearCode`)
          (`self.SetButton` 9 true)
          (elif (or (and (<= _returnvalue_2 9) (> _returnvalue_2 0)) (`KismetStringLibrary.EqualEqual_StrStr` _returnvalue "0"))
            (`self.ClickNumber` _returnvalue_2)))))))

(event `self.ReceiveBeginPlay`
  (`self.ClearCode`))

(event `WrongCode`
  (set `self.bIgnoreInputs` true)
  (`/Game/TrickPhotography/Programmers/Core/BaseClasses/CustomMacros.DelayableForLoop` 0 6 :!label _label
    (:`LoopBody`
      (`PrimitiveComponent.SetMaterial` (`self.FilterSkeletalMesh`) 1 (`self.FailMat`))
      (`KismetSystemLibrary.Delay` 0.2)
      (`PrimitiveComponent.SetMaterial` (`self.FilterSkeletalMesh`) 1 "/Game/Developers/cu1us/MI_PureUnlit_Blue.MI_PureUnlit_Blue")
      (`KismetSystemLibrary.Delay` 0.2)
      (goto _label :!via `CountUp`))
    (:`Completed`
      (`self.ClearCode`)
      (set `self.bIgnoreInputs` false))))

(fn `ClearCode`
  (set `self.InputtedCode` "")
  (`self.RefreshDisplay`))

(fn `ClickNumber`
  (params (Number :type Integer))
  (bind _correctcode (`self.CorrectCode`))
  (`self.SetButton` (`KismetMathLibrary.SelectInt` 10 (- Number 1) (== Number 0)) true)
  (bind _output_get (set `self.InputtedCode` (`KismetStringLibrary.Concat_StrStr` (`self.InputtedCode`) (`KismetStringLibrary.Conv_IntToString` Number))))
  (`self.RefreshDisplay`)
  (if (`KismetStringLibrary.EqualEqual_StrStr` _output_get _correctcode)
    (`self.ConfirmCode` :!label _label)
    (elif (>= (`KismetStringLibrary.Len` _output_get) (`KismetStringLibrary.Len` _correctcode))
      (goto _label))))

(fn `ConfirmCode`
  (bind _inputtedcode (`self.InputtedCode`))
  (if (`KismetStringLibrary.IsEmpty` _inputtedcode)
    _
    (elif (`KismetStringLibrary.EqualEqual_StrStr` _inputtedcode (`self.CorrectCode`))
      (`self.Open`)
      (else
        (`self.WrongCode`)))))

(fn `GetInteractionType`
  (params (bIsCammy :type Boolean) (HitComponent :type "PrimitiveComponent Object Reference"))
  (returns (Type :type "/Game/TrickPhotography/Programmers/Enums/EPlayerInteractionState Enum") (CustomInteractTooltip :type Text))
  (return "NewEnumerator0" ""))

(fn `HoverOngoing`
  (params (HeldItem :type "PickupableInterface Interface") (HitComponent :type "PrimitiveComponent Object Reference"))
  (returns (bIsInteractable :type Boolean))
  (return false))

(fn `HoverStart`
  (params (HeldItem :type "PickupableInterface Interface") (HitComponent :type "PrimitiveComponent Object Reference") (bIsCammy :type Boolean))
  (returns (bIsInteractable :type Boolean))
  (return false))

(fn `Open`
  (set `self.bIgnoreInputs` true)
  (`self.OnActivated`)
  (`KismetSystemLibrary.PrintString` "Correct PIN entered!" true true (struct :`R` 0.296638 :`G` 1.0 :`A` 1.0) 3.0))

(fn `SetButton`
  (params (ButtonIndex :type Integer) (bPressed :type Boolean))
  (set `self.HeldButton` (`KismetMathLibrary.SelectInt` ButtonIndex -1 bPressed))
  (bind _asabp_keypad (cast `/Game/TrickPhotography/Art/Enviroment/Meshes/ABP_Keypad` (`SkeletalMeshComponent.GetAnimInstance` (`self.FilterSkeletalMesh`)))
    (:`then`
      (`/Game/TrickPhotography/Art/Enviroment/Meshes/ABP_Keypad.SetKey` _asabp_keypad ButtonIndex bPressed)
      (`KismetSystemLibrary.PrintText` (`|FormatText` "{Index}: {Pressed}" ButtonIndex bPressed)))
    (:`CastFailed`
      (`KismetSystemLibrary.PrintString` "Failed cast to anim instance"))))

(fn `UserConstructionScript`)