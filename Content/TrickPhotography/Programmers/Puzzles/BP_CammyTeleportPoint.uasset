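; BP_CammyTeleportPoint is an interactable puzzle point, prompted as "Enter Vent", that moves the Cammy character to another location.
; When Cammy interacts while it is usable, it either drives her location and rotation along a spline with a timeline or snaps her to a target point.
; A Teleporting flag on Cammy blocks re-triggering during spline travel.
; Hovering as Cammy shows a hint highlight, cleared on hover end.
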(event `/Game/TrickPhotography/Programmers/Core/Interfaces/BPI_Interactable.InteractStart`
  (params (HeldItem :type "PickupableInterface Interface") (bIsCammy :type Boolean) (HitComponent :type "PrimitiveComponent Object Reference"))
  (bind _teleportingactor (`self.TeleportingActor`))
  (if (and bIsCammy (`self.bUsable`))
    (bind _asmain_player_controller (cast `/Game/TrickPhotography/Programmers/Core/Player/MainPlayerController` (`GameplayStatics.GetPlayerController` 0)))
    (bind _output_get (set `self.TeleportingActor` (`/Game/TrickPhotography/Programmers/Core/Player/MainPlayerController.CammyChar` _asmain_player_controller)))
    (if (`/Game/TrickPhotography/Programmers/Core/Player/BP_CammyCharacter.bTeleporting` _output_get)
      _
      (elif (`self.bSplineMovement`)
        (set `self.TeleportingActorStartLoc` (`self.K2_GetActorLocation` _teleportingactor))
        (`/Game/TrickPhotography/Programmers/Core/Player/BP_CammyCharacter.SetTeleporting` _teleportingactor true)
        (bind (_direction _timer) (`Timeline|LerpTimer` :!via `PlayFromStart`)
          (:`Update`
            (bind (_returnvalue_location _returnvalue_rotation) (`KismetMathLibrary.BreakTransform` (`SplineComponent.GetTransformAtTime` (`self.Spline`) _timer "World" false false)))
            (`self.K2_SetActorLocationAndRotation` (`self.TeleportingActor`) _returnvalue_location _returnvalue_rotation false false))
          (:`Finished`
            (`/Game/TrickPhotography/Programmers/Core/Player/BP_CammyCharacter.SetTeleporting` (`self.TeleportingActor`) false)))
        (else
          (`self.K2_SetActorLocation` (`self.TeleportingActor`) (`self.K2_GetActorLocation` (`self.TargetPoint`)) false true))))))

(event `/Game/TrickPhotography/Programmers/Core/Interfaces/BPI_Interactable.HoverEnd`
  (params (HeldItem :type "PickupableInterface Interface") (bIsCammy :type Boolean))
  (if bIsCammy
    (`self.SetPPMHighlight` "None")))

(fn `GetInteractionType`
  (params (bIsCammy :type Boolean) (HitComponent :type "PrimitiveComponent Object Reference"))
  (returns (Type :type "/Game/TrickPhotography/Programmers/Enums/EPlayerInteractionState Enum") (CustomInteractTooltip :type Text))
  (if bIsCammy
    (return "NewEnumerator5" "Enter Vent")
    (else
      (return "NewEnumerator5" ""))))

(fn `HoverOngoing`
  (params (HeldItem :type "PickupableInterface Interface") (HitComponent :type "PrimitiveComponent Object Reference"))
  (returns (bIsInteractable :type Boolean))
  (return false))

(fn `HoverStart`
  (params (HeldItem :type "PickupableInterface Interface") (HitComponent :type "PrimitiveComponent Object Reference") (bIsCammy :type Boolean))
  (returns (bIsInteractable :type Boolean))
  (if bIsCammy
    (`self.SetPPMHighlight` "HighlightHint")
    (return false)))

(fn `UserConstructionScript`)