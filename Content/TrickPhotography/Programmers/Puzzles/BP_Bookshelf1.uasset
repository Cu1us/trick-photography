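; BP_Bookshelf1 is a puzzle bookshelf that slides to an offset location while its book slots hold the correct books.
; On BeginPlay it binds to each slot's book-attached event, then compares held IDs against CorrectIDs in order on each update.
; A match fires OnActivated and opens the shelf, while a mismatch closes it.
; Tick drives a clamped one-second lerp between closed and open positions, and debug prints remain.
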(event `self.ReceiveBeginPlay`
  (bind _returnvalue (`self.K2_GetActorLocation`))
  (set `self.ClosedLocation` _returnvalue)
  (set `self.OpenOffsetLocation` (+ _returnvalue (`self.OpenOffsetLocation`)))
  (for _array_element (`self.BookSlots`)
    (add `/Game/TrickPhotography/Programmers/Puzzles/BP_BookSlot.OnAttachedBook` _array_element (delegate `SlotsUpdated`))))

(event `SlotsUpdated`
  (bind _matching (`self.CheckForMatch`))
  (if _matching
    (`self.OnActivated`)
    (`KismetSystemLibrary.PrintString` "correct solution inputted!!!" true true (struct :`R` 1.0 :`G` 0.958984 :`A` 1.0) 6.0)
    (set `self.bOpen` true)
    (else
      (set `self.bOpen` false))))

(event `self.ReceiveTick`
  (params (DeltaSeconds :type "Float (single-precision)"))
  (if (`self.bOpen`)
    (set `self.LerpTimer` (`KismetMathLibrary.FClamp` (+ (`self.LerpTimer`) DeltaSeconds)))
    (else
      (set `self.LerpTimer` (`KismetMathLibrary.FClamp` (- (`self.LerpTimer`) DeltaSeconds)))))
  (`self.K2_SetActorLocation` (`KismetMathLibrary.VLerp` (`self.ClosedLocation`) (`self.OpenOffsetLocation`) (`self.LerpTimer`))))

(fn `CheckForMatch`
  (returns (Matching :type Boolean))
  (locals (IsMatch :type Boolean :default true))
  (set `local.IsMatch` true)
  (for _index (range (`KismetArrayLibrary.Array_Length` (`self.CorrectIDs`)))
    (bind _heldid (`/Game/TrickPhotography/Programmers/Puzzles/BP_BookSlot.HeldID` (`|GetArrayItem` (`self.BookSlots`) _index)))
    (`KismetSystemLibrary.PrintString` _heldid true true (struct :`G` 1.0 :`B` 0.028208 :`A` 1.0))
    (if (not (== _heldid (`|GetArrayItem` (`self.CorrectIDs`) _index)))
      (set `local.IsMatch` false)
      (break)))
  (return (`local.IsMatch`)))

(fn `UserConstructionScript`)