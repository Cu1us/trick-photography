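; Puzzle text actor that shows its TextRender while its ActivationSource is activated, except during photos.
; BeginPlay binds Activate and Deactivate to the source's events.
; OnAnyPhoto and OnAnyPhotoFinished set and clear a filter-hide flag.
; All four events call UpdateVisibility, which combines activation state with that flag, without propagating visibility to child components.
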(event `self.ReceiveBeginPlay`
  (bind _activationsource (`self.ActivationSource`))
  (add `/Game/TrickPhotography/Programmers/Core/BaseClasses/BP_ActivatorBase.OnActivated` _activationsource (delegate `/Game/TrickPhotography/Programmers/Core/Interfaces/BPI_Activatable.Activate`))
  (add `/Game/TrickPhotography/Programmers/Core/BaseClasses/BP_ActivatorBase.OnDeactivated` _activationsource (delegate `/Game/TrickPhotography/Programmers/Core/Interfaces/BPI_Activatable.Deactivate`)))

(event `/Game/TrickPhotography/Programmers/Core/Interfaces/BPI_Activatable.Activate`
  (`self.UpdateVisibility`))

(event `/Game/TrickPhotography/Programmers/Core/Interfaces/BPI_Activatable.Deactivate`
  (`self.UpdateVisibility`))

(event `FilterableInterface.OnAnyPhoto`
  (set `self.bIsHiddenDueToFilter` true)
  (`self.UpdateVisibility`))

(event `FilterableInterface.OnAnyPhotoFinished`
  (set `self.bIsHiddenDueToFilter` false)
  (`self.UpdateVisibility`))

(fn `UserConstructionScript`)