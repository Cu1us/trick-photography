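; BP_BreakerBox is an interactable puzzle breaker that players toggle on and off, with a click sound, debug print and hover highlight.
; An optional dependency ignores interaction unless another referenced breaker is activated.
; Activate and Deactivate extend the parent's logic by swapping the box's material to show its state.
; It can start activated, applied one tick after BeginPlay.
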(event `self.ReceiveBeginPlay`
  (`KismetSystemLibrary.DelayUntilNextTick`)
  (if (`self.bActivatedOnBegin`)
    (`self.Activate`)))

(event `/Game/TrickPhotography/Programmers/Core/Interfaces/BPI_Interactable.InteractStart`
  (params (HeldItem :type "PickupableInterface Interface") (bIsCammy :type Boolean) (HitComponent :type "PrimitiveComponent Object Reference"))
  (if (`self.bRequireOtherBreaker`)
    (if (`self.IsActivated` (`self.OtherBreaker`))
      (`GameplayStatics.PlaySound2D` "/Game/TrickPhotography/Audio/MS_ButtonClick.MS_ButtonClick" 1.0 1.0 0.0 null null :!label _label)
      (if (`self.bIsActivated`)
        (`self.Deactivate`)
        (`KismetSystemLibrary.PrintString` "Breaker OFF" true true (struct :`R` 0.296007 :`G` 0.12533 :`B` 0.104322 :`A` 1.0))
        (else
          (`self.Activate`)
          (`KismetSystemLibrary.PrintString` "Breaker ON" true true (struct :`R` 0.075843 :`G` 1.0 :`A` 1.0)))))
    (else
      (goto _label))))

(event `/Game/TrickPhotography/Programmers/Core/Interfaces/BPI_Interactable.HoverEnd`
  (params (HeldItem :type "PickupableInterface Interface") (bIsCammy :type Boolean))
  (`self.SetPPMHighlight` "None"))

(fn `Activate`
  (`parent.Activate`)
  (`FilterStaticMeshComponent.SetMainMaterial` (`self.BreakerBox`) "/Game/TrickPhotography/Art/Materials/BreakerBox/M_BreakerBox.M_BreakerBox"))

(fn `Deactivate`
  (`parent.Deactivate`)
  (`FilterStaticMeshComponent.SetMainMaterial` (`self.BreakerBox`) "/Game/TrickPhotography/Art/Materials/BreakerBox/M_Breakerboxoff.M_Breakerboxoff"))

(fn `GetInteractionType`
  (params (bIsCammy :type Boolean) (HitComponent :type "PrimitiveComponent Object Reference"))
  (returns (Type :type "/Game/TrickPhotography/Programmers/Enums/EPlayerInteractionState Enum") (CustomInteractTooltip :type Text))
  (return "NewEnumerator0" ""))

(fn `HoverOngoing`
  (params (HeldItem :type "PickupableInterface Interface") (HitComponent :type "PrimitiveComponent Object Reference"))
  (returns (bIsInteractable :type Boolean))
  (return false))

(fn `HoverStart`
  (params (HeldItem :type "PickupableInterface Interface") (HitComponent :type "PrimitiveComponent Object Reference") (bIsCammy :type Boolean))
  (returns (bIsInteractable :type Boolean))
  (`self.SetPPMHighlight` "HighlightPickup")
  (return false))

(fn `UserConstructionScript`)