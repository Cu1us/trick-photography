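; Possessable vault puzzle where the player turns a dial to rotate combination discs, randomized at BeginPlay.
; Interacting as non-Cammy possesses the vault; IA_ExitPuzzle returns control to the main character.
; RotateWheel recursively drags the next disc when pins meet, with tick audio and step positions read from each disc's yaw.
; Solution rings change material when their disc reaches the correct rotation, but CheckForCorrectSolution is an empty stub.
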(event `EnhancedInput|/Game/TrickPhotography/Programmers/Core/Inputs/Vault/IA_TurnDial`
  (params (ActionValue :type "Float (double-precision)") (ElapsedSeconds :type "Float (double-precision)") (TriggeredSeconds :type "Float (double-precision)") (InputAction :type "InputAction Object Reference" :default "/Game/TrickPhotography/Programmers/Core/Inputs/Vault/IA_TurnDial.IA_TurnDial"))
  (:`Triggered`
    (`self.RotateWheel` 0 (== ActionValue 1.0))))

(event `self.ReceiveBeginPlay`
  (`self.RandomizeDiscPositions`))

(event `self.ReceiveControllerChanged`
  (params (OldController :type "Controller Object Reference") (NewController :type "Controller Object Reference"))
  (bind _asmain_player_controller (cast `/Game/TrickPhotography/Programmers/Core/Player/MainPlayerController` NewController))
  (`EnhancedInputSubsystemInterface.AddMappingContext` (pcsubsystem `EnhancedInputLocalPlayerSubsystem` _asmain_player_controller) "/Game/TrickPhotography/Programmers/Core/Inputs/Vault/IMC_Vault.IMC_Vault" 2 (struct)))

(event `/Game/TrickPhotography/Programmers/Core/Interfaces/BPI_Interactable.InteractStart`
  (params (HeldItem :type "PickupableInterface Interface") (bIsCammy :type Boolean))
  (if (not bIsCammy)
    (bind _asmain_player_controller (cast `/Game/TrickPhotography/Programmers/Core/Player/MainPlayerController` (`GameplayStatics.GetPlayerController` 0)))
    (`Controller.Possess` _asmain_player_controller self)
    (`KismetSystemLibrary.PrintString` "Entered puzzle" true true (struct :`G` 0.446832 :`B` 1.0 :`A` 1.0) 2.0 "vault")))

(event `EnhancedInput|/Game/TrickPhotography/Programmers/Core/Inputs/Vault/IA_ExitPuzzle`
  (params (ActionValue :type Boolean) (ElapsedSeconds :type "Float (double-precision)") (TriggeredSeconds :type "Float (double-precision)") (InputAction :type "InputAction Object Reference" :default "/Game/TrickPhotography/Programmers/Core/Inputs/Vault/IA_ExitPuzzle.IA_ExitPuzzle"))
  (:`Triggered`
    (bind _asmain_player_controller (cast `/Game/TrickPhotography/Programmers/Core/Player/MainPlayerController` (`GameplayStatics.GetPlayerController` 0)))
    (`EnhancedInputSubsystemInterface.RemoveMappingContext` (pcsubsystem `EnhancedInputLocalPlayerSubsystem` _asmain_player_controller) "/Game/TrickPhotography/Programmers/Core/Inputs/Vault/IMC_Vault.IMC_Vault" (struct))
    (`/Game/TrickPhotography/Programmers/Core/Player/MainPlayerController.PossessMainCharacter` _asmain_player_controller)
    (`KismetSystemLibrary.PrintString` "Exited puzzle" true true (struct :`G` 0.446832 :`B` 1.0 :`A` 1.0) 2.0 "vault")))

(fn `EnableSolutionRing`
  (params (Index :type Integer) (Enabled :type Boolean))
  (bind _returnvalue (select `int` Index :`0` (`self.Small`) :`1` (`self.Medium`) :`2` (`self.Big`)))
  (`/Engine/EditorBlueprintResources/StandardMacros.IsValid` _returnvalue
    (:`Is Valid`
      (`PrimitiveComponent.SetMaterial` _returnvalue 0 (select `bool` Enabled :`false` (`self.SolutionRingIncorrectMaterial`) :`true` (`self.SolutionRingCorrectMaterial`))))))

(fn `RandomizeDiscPositions`
  (for _index (range (`SceneComponent.GetNumChildrenComponents` (`self.Discs`)))
    (`self.SetWheelRotation` _index (`KismetMathLibrary.RandomIntegerInRange` 0 (- (`self.Steps`) 1)))))

(fn `RotateWheel`
  (params (WheelIndex :type Integer) (Clockwise :type Boolean))
  (bind _returnvalue (+ WheelIndex 1))
  (bind _realpinrotation (`self.GetRealPinLocation` WheelIndex)
    (:`Then`
      (bind _realpinrotation_2 (`self.GetRealPinLocation` _returnvalue)
        (:`Then`
          (if (== (`KismetMathLibrary.SelectInt` _realpinrotation_2 (`self.AddWithModulo` _realpinrotation_2 1) Clockwise) _realpinrotation)
            (`self.RotateWheel` _returnvalue Clockwise)))
        (:`Failed`
          _))
      (bind _wheelrotation (`self.GetWheelRotation` WheelIndex)
        (:`then`
          (`self.SetWheelRotation` WheelIndex (`self.AddWithModulo` _wheelrotation (`KismetMathLibrary.SelectInt` 1 -1 Clockwise))))
        (:`Failed`
          _))
      (`self.PlayWheelTick` WheelIndex))))

(fn `UserConstructionScript`)