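; Puzzle slot for books that shows a highlight mesh while it is empty and the player holds a BP_Book.
; It tracks held books through the main character's left-hand state change event and occupancy through book overlaps.
; Occupancy also switches the box's Camera channel response, ignoring it when filled and blocking it when empty.
; SetRegisteredBook stores the book ID and fires the OnAttachedBook dispatcher.
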(event `self.ReceiveBeginPlay`
  (bind _asmain_player_controller (cast `/Game/TrickPhotography/Programmers/Core/Player/MainPlayerController` (`GameplayStatics.GetPlayerController` 0)))
  (bind _output_get (set `self.Main Char` (`/Game/TrickPhotography/Programmers/Core/Player/MainPlayerController.MainChar` _asmain_player_controller)))
  (add `/Game/TrickPhotography/Programmers/Core/Player/BP_MainCharacter.LHandStateChangeEvent` _output_get (delegate `ToggleHighlight`))
  (set `self.bEmpty` (== (`KismetArrayLibrary.Array_Length` (`PrimitiveComponent.GetOverlappingActors` (`self.Box`) "/Game/TrickPhotography/Programmers/Pickups/BP_Book.BP_Book_C")) 0)))

(event `ToggleHighlight`
  (cast `/Game/TrickPhotography/Programmers/Pickups/BP_Book` (`/Game/TrickPhotography/Programmers/Core/Player/BP_MainCharacter.HeldObject` (`self.Main Char`))
    (:`then`
      (set `self.bPlayerHoldsBook` true))
    (:`CastFailed`
      (set `self.bPlayerHoldsBook` false)))
  (`self.UpdateHighlightState`))

(event `self.ReceiveActorBeginOverlap`
  (params (OtherActor :type "Actor Object Reference"))
  (cast `/Game/TrickPhotography/Programmers/Pickups/BP_Book` OtherActor)
  (`PrimitiveComponent.SetCollisionResponseToChannel` (`self.Box`) "ECC_Camera" "ECR_Ignore")
  (set `self.bEmpty` false)
  (`self.UpdateHighlightState` :!label _label))

(event `self.ReceiveActorEndOverlap`
  (params (OtherActor :type "Actor Object Reference"))
  (cast `/Game/TrickPhotography/Programmers/Pickups/BP_Book` OtherActor)
  (`PrimitiveComponent.SetCollisionResponseToChannel` (`self.Box`) "ECC_Camera" "ECR_Block")
  (set `self.bEmpty` true)
  (goto _label))

(event `SetRegisteredBook`
  (params (ID :type String))
  (set `self.HeldID` ID)
  (`self.OnAttachedBook`))

(fn `UpdateHighlightState`
  (if (and (`self.bEmpty`) (`self.bPlayerHoldsBook`))
    (`SceneComponent.SetVisibility` (`self.FilterStaticMesh`) true false)
    (else
      (`SceneComponent.SetVisibility` (`self.FilterStaticMesh`) false false))))

(fn `UserConstructionScript`)