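; BP_CammyKnockablePot is a puzzle prop that lets the Cammy character knock a destructible pot loose.
; It wraps a BP_DestructiblePot child actor and turns off its physics simulation on BeginPlay to hold it in place.
; The first overlap of Collider by BP_CammyCharacter sets a one-shot Activated flag and enables physics on the pot.
; Debug strings print on activation and on failed pot casts.
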(event `self.ReceiveBeginPlay`
  (bind _asbp_destructible_pot (cast `/Game/TrickPhotography/Programmers/Puzzles/BP_DestructiblePot` (`ChildActorComponent.ChildActor` (`self.Pot`)))
    (:`then`
      (`PrimitiveComponent.SetSimulatePhysics` (`/Game/TrickPhotography/Programmers/Puzzles/BP_DestructiblePot.Pot` _asbp_destructible_pot) false))
    (:`CastFailed`
      (`KismetSystemLibrary.PrintString` "dag nabbit" true true (struct :`G` 0.66 :`B` 1.0 :`A` 1.0) 12.0 :!label _label))))

(event `self.Collider.OnComponentBeginOverlap`
  (params (OverlappedComponent :type "PrimitiveComponent Object Reference") (OtherActor :type "Actor Object Reference") (OtherComp :type "PrimitiveComponent Object Reference") (OtherBodyIndex :type Integer) (bFromSweep :type Boolean) (SweepResult :type "HitResult Structure (by ref)"))
  (if (not (`self.bActivated`))
    (cast `/Game/TrickPhotography/Programmers/Core/Player/BP_CammyCharacter` OtherActor)
    (set `self.bActivated` true)
    (bind _asbp_destructible_pot (cast `/Game/TrickPhotography/Programmers/Puzzles/BP_DestructiblePot` (`ChildActorComponent.ChildActor` (`self.Pot`)))
      (:`then`
        (`PrimitiveComponent.SetSimulatePhysics` (`/Game/TrickPhotography/Programmers/Puzzles/BP_DestructiblePot.Pot` _asbp_destructible_pot) true)
        (`KismetSystemLibrary.PrintString` "yaheow"))
      (:`CastFailed`
        (goto _label)))))

(fn `UserConstructionScript`)