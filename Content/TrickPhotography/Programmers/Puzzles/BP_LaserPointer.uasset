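; BP_LaserPointer is a puzzle laser emitter that lights any BP_LaserMatch actor its beam hits.
; While Enabled, it runs a short forward line trace on the Visibility channel from its root every Tick.
; SetLaserPoints feeds the trace start and impact point into the Beam Niagara component's position variables.
; A hit on a BP_LaserMatch then calls its Light function.
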(event `self.ReceiveTick`
  (params (DeltaSeconds :type "Float (single-precision)"))
  (bind (_returnvalue_location _returnvalue_rotation) (`KismetMathLibrary.BreakTransform` (`SceneComponent.K2_GetComponentToWorld` (`self.DefaultSceneRoot`))))
  (if (`self.bEnabled`)
    (bind _outhit (`KismetSystemLibrary.LineTraceSingle` _returnvalue_location (+ _returnvalue_location (* (`KismetMathLibrary.GetForwardVector` _returnvalue_rotation) 1000.0)) "TraceTypeQuery1"))
    (bind (_bblockinghit _binitialoverlap _time _distance _location _impactpoint _normal _impactnormal _physmat _hitactor _hitcomponent _hitbonename _bonename _hititem _elementindex _faceindex _tracestart) (`GameplayStatics.BreakHitResult` _outhit))
    (`self.SetLaserPoints` _tracestart _impactpoint)
    (bind _asbp_laser_match (cast `/Game/TrickPhotography/Programmers/Puzzles/BP_LaserMatch` _hitactor))
    (`/Game/TrickPhotography/Programmers/Puzzles/BP_LaserMatch.Light` _asbp_laser_match)))

(fn `SetLaserPoints`
  (params (Start :type "Vector Structure") (End :type "Vector Structure"))
  (bind _beam (`self.Beam`))
  (`NiagaraComponent.SetVariablePosition` _beam "Start" Start)
  (`NiagaraComponent.SetVariablePosition` _beam "End" End))

(fn `UserConstructionScript`)