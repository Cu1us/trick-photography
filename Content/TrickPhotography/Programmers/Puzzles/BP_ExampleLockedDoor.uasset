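; Example locked door puzzle interactable that responds to a key pickup held by the player.
; On interact start, it casts the held item to Pickup and compares its PickupID with RequiredKeyID.
; A match toggles FilterStaticMesh visibility without propagating to children; a wrong or missing key only prints a debug message.
; Interact end does nothing, and construction just calls the parent.
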(event `/Game/TrickPhotography/Programmers/Core/Interfaces/BPI_Interactable.InteractStart`
  (params (HeldItem :type "PickupableInterface Interface"))
  (bind _aspickup (cast `Pickup` HeldItem)
    (:`then`
      (if (== (`self.RequiredKeyID`) (`Pickup.PickupID` _aspickup))
        (`SceneComponent.ToggleVisibility` (`self.FilterStaticMesh`) false)
        (else
          (`KismetSystemLibrary.PrintString` "wrong key"))))
    (:`CastFailed`
      (`KismetSystemLibrary.PrintString` "door is locked"))))

(event `/Game/TrickPhotography/Programmers/Core/Interfaces/BPI_Interactable.InteractEnd`)

(fn `UserConstructionScript`
  (`parent.UserConstructionScript`))